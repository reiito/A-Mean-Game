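; Player controller that owns the character's spawn point, respawning, capped dead-body spawning and per-level rules.
; On respawn it bumps the GameInstance death counter, possesses a new BP_Character, reapplies invincibility and unlocks, and runs the PlayerSpawner when at the initial point.
; Unlocks and the invincibility cheat come from the GameInstance.
; Editor-only debug keys respawn, restart, clear the save, or jump to the level end or cow collectible.
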(event `self.ReceiveBeginPlay`
  (bind _returnvalue (`self.GetTransform` (`GameplayStatics.GetPlayerPawn` 0)))
  ;[1 1 1] Startup
  (`self.Initialize`)
  (`self.UpdateSpawnPoint` _returnvalue)
  (set `self.InitialSpawnPoint` _returnvalue))

(event `Key|R`
  (params (Key :type "Key Structure"))
  ;[1 1 1] Restart Key
  (:`Pressed`
    (if (`PlayerBPFL.InEditor`) :!label _label
      (`/Game/Game/BP_GameMode.Respawn` (`self.GameMode`)))))

(event `Key|Gamepad_FaceButton_Top`
  (params (Key :type "Key Structure"))
  ;[1 1 1] Restart Key
  (:`Pressed`
    (goto _label)))

(event `Key|Apostrophe`
  (params (Key :type "Key Structure"))
  (:`Pressed`
    (if (`PlayerBPFL.InEditor`) :!label _label_2
      (`self.RestartGame`))))

(event `Key|Gamepad_Special_Left`
  (params (Key :type "Key Structure"))
  (:`Pressed`
    (goto _label_2)))

(event `Key|Delete`
  (params (Key :type "Key Structure"))
  (:`Pressed`
    (if (`PlayerBPFL.InEditor`)
      (`/Game/Game/BP_GameInstance.ClearSave` (`self.GameInstance`)))))

(event `Key|End`
  (params (Key :type "Key Structure"))
  (:`Pressed`
    (if (`PlayerBPFL.InEditor`)
      (bind _outactors (`GameplayStatics.GetAllActorsOfClass` "/Game/LevelCreation/_LevelRequirements/BP_LevelEnd.BP_LevelEnd_C"))
      (bind _output (`|GetArrayItem` _outactors))
      (`/Engine/EditorBlueprintResources/StandardMacros.IsValid` _output
        (:`Is Valid`
          (bind _pickup (`/Game/LevelCreation/Pickups/BP_Pickup.Pickup` _output))
          (set `self.PlayerSpawnPoint` (`KismetMathLibrary.MakeTransform` (+ (`SceneComponent.K2_GetComponentLocation` _pickup) (* (`SceneComponent.GetForwardVector` _pickup) 200.0) (0.0 0.0 150.0))))
          (`/Game/Game/BP_GameMode.Respawn` (`self.GameMode`)))))))

(event `Key|PageDown`
  (params (Key :type "Key Structure"))
  (:`Pressed`
    (if (`PlayerBPFL.InEditor`)
      (bind _outactors (`GameplayStatics.GetAllActorsOfClass` "/Game/LevelCreation/Pickups/BP_CowCollectible.BP_CowCollectible_C"))
      (bind _output (`|GetArrayItem` _outactors))
      (`/Engine/EditorBlueprintResources/StandardMacros.IsValid` _output
        (:`Is Valid`
          (set `self.PlayerSpawnPoint` (`KismetMathLibrary.MakeTransform` (+ (`SceneComponent.K2_GetComponentLocation` (`/Game/LevelCreation/Pickups/BP_Pickup.Pickup` _output)) (0.0 0.0 150.0))))
          (`/Game/Game/BP_GameMode.Respawn` (`self.GameMode`)))))))

(fn `AssignInvincibilityToPlayer`
  (`/Game/Player/BP_Character.SetInvincibility` (`self.CurrentCharacter`) (`self.PlayerInvincible`)))

(fn `AssignUnlockablesToPlayer`
  (params (Reupdate :type Boolean))
  (`|ExecutionSequence`
    (:`then_0`
      ;[1 1 1] Recheck game instance to see if unlocks have changed
      (if (`local.Reupdate`)
        (`self.GetInstanceUnlockables`)))
    (:`then_1`
      (`/Game/Player/BP_Character.SetupUnlockables` (`self.CurrentCharacter`) (`self.PlayerCanDoubleJump`) (`self.PlayerCanSprint`) (`self.PlayerInvincible`)))))

(fn `GetInstanceUnlockables`
  (set `self.PlayerCanSprint` (`/Game/Game/BP_GameInstance.SprintUnlocked` (`self.GameInstance`)))
  (set `self.PlayerCanDoubleJump` (`/Game/Game/BP_GameInstance.DoubleJumpUnlocked` (`self.GameInstance`)))
  (set `self.PlayerInvincible` (`/Game/Game/BP_GameInstance.Invincible` (`self.GameInstance`))))

(fn `Initialize`
  (`self.SetupReferences`)
  (`self.AssignUnlockablesToPlayer` true))

(fn `ReassignParamsOnRespawn`
  (`self.AssignInvincibilityToPlayer`)
  (`self.AssignUnlockablesToPlayer` false))

(fn `RestartGame`
  (`/Game/Game/BP_GameInstance.ResetInstance` (`self.GameInstance`))
  (`GameplayStatics.OpenLevel` "LVL_MainMenu"))

(fn `SetLevelParams`
  (params (CanSpawnDeadBody :type Boolean) (Invincible :type Boolean) (MaxDeadBodies :type Integer))
  (set `self.CanSpawnDeadBody` CanSpawnDeadBody)
  (set `self.PlayerInvincible` Invincible)
  (set `self.MaxDeadBodies` MaxDeadBodies)
  ;[1 1 1] Player not set to invincible, check if cheat used
  (if (not (`local.Invincible`))
    (set `self.PlayerInvincible` (`/Game/Game/BP_GameInstance.Invincible` (`self.GameInstance`)))))

(fn `SetupReferences`
  (bind _asbp_character (cast `/Game/Player/BP_Character` (`GameplayStatics.GetPlayerPawn` 0)))
  (set `self.CurrentCharacter` _asbp_character)
  (bind _asbp_game_mode (cast `/Game/Game/BP_GameMode` (`GameplayStatics.GetGameMode`)))
  (set `self.GameMode` _asbp_game_mode)
  (bind _asbp_game_instance (cast `/Game/Game/BP_GameInstance` (`GameplayStatics.GetGameInstance`)))
  (set `self.GameInstance` _asbp_game_instance))

(fn `SpawnCharacter`
  (bind _playerspawner (`self.PlayerSpawner`))
  ;[1 1 1] Update death count
  (`/Game/Game/BP_GameInstance.IncrementDeathCounter` (`self.GameInstance`))
  ;[1 1 1] Spawn character pawn
  (bind _returnvalue (`|SpawnActorFromClass` "/Game/Player/BP_Character.BP_Character_C" (`self.PlayerSpawnPoint`) "Undefined" "OverrideRootScale" null null))
  (set `self.CurrentCharacter` _returnvalue)
  (`self.ReassignParamsOnRespawn`)
  (`self.Possess` _returnvalue)
  ;[1 1 1] Check if player spawner is being used. If so attach character and run its behaviour
  (`/Engine/EditorBlueprintResources/StandardMacros.IsValid` _playerspawner
    (:`Is Valid`
      (if (== (`self.PlayerSpawnPoint`) (`self.InitialSpawnPoint`))
        (`/Game/Player/BP_CharacterSpawner.AttachCharacter` _playerspawner (`self.CurrentCharacter`))
        (`/Game/Player/BP_CharacterSpawner.RunBehaviour` _playerspawner)))))

(fn `SpawnDeadBody`
  (bind _currentcharacter (`self.CurrentCharacter`))
  (bind (_deathtransform_location _deathtransform_rotation _deathtransform_scale) (`KismetMathLibrary.BreakTransform` (`/Game/Player/BP_Character.DeathTransform` _currentcharacter)))
  (if (and (`self.CanSpawnDeadBody`) (< (`self.NumDeadBodies`) (`self.MaxDeadBodies`)))
    (`|SpawnActorFromClass` "/Game/Player/BP_DeadCharacter.BP_DeadCharacter_C" (`KismetMathLibrary.MakeTransform` (+ _deathtransform_location (`self.DeadBodySpawnOffset`)) (`SceneComponent.K2_GetComponentRotation` (`Character.Mesh` _currentcharacter)) _deathtransform_scale) "Undefined" "OverrideRootScale" null null)
    (`/Engine/EditorBlueprintResources/StandardMacros.IncrementInt` (`self.NumDeadBodies`))))

(fn `UpdateSpawnPoint`
  (params (NewSpawnPoint :type "Transform Structure"))
  (set `self.PlayerSpawnPoint` NewSpawnPoint))

(fn `UserConstructionScript`)