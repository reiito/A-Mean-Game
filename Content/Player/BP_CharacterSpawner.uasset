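; Character spawner that stages the player's entrance, with input disabled and the camera detached at a fixed start position.
; RunBehaviour raises the spawner on a lerp timeline while updating shadow opacity, then after a delay glides the camera behind the character.
; When the zoom ends, it reattaches the camera, restores input and triggers the LevelTracker intro once.
; The character comes from a child actor or AttachCharacter, and the rise can be reversed.
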(event `self.ReceiveBeginPlay`
  ;[1 1 1] Startup
  (`self.SetupParameters`)
  (`/Game/Game/BP_Macros.SetupLerpTimeline` (`self.MoveSpawnerAnimation`) "/Game/Data/CURVEs/CURVE_LinearLerp.CURVE_LinearLerp" (`self.AnimationSpeed`)
    (:`__`
      (`/Game/Game/BP_Macros.SetupLerpTimeline` (`self.ZoomIntoCharacterAnimation`) "/Game/Data/CURVEs/CURVE_LinearLerp.CURVE_LinearLerp" (`self.ZoomIntoCharacterSpeed`)))))

(event `RunBehaviour`
  ;[1 1 1] Behaviour
  (`self.MoveSpawnerUp`)
  (`KismetSystemLibrary.Delay` (`self.MoveUpFinishDelay`))
  (`self.ZoomInAndEnableCharacter`))

(event `ZoomInAndEnableCharacter`
  (bind _player (`self.Player`))
  (bind _player_2 (`self.Player`))
  ;[1 1 1] Zoom into character after all animations finish then enable controls again
  (`Timeline|ZoomIntoCharacterAnimation`
    (:`Update`
      (`/Engine/EditorBlueprintResources/StandardMacros.IsValid` _player_2
        (:`Is Valid`
          (`/Game/Game/BP_Macros.MoveComponent` (`/Game/Player/BP_Character.Camera` _player_2) (`SceneComponent.K2_GetComponentLocation` (`self.CameraStartPosition`)) (`SceneComponent.K2_GetComponentLocation` (`/Game/Player/BP_Character.BehindTransform` _player_2)) (`self.ZoomIntoCharacterAnimation`)))))
    (:`Finished`
      (`/Engine/EditorBlueprintResources/StandardMacros.IsValid` _player
        (:`Is Valid`
          (`/Game/Player/BP_Character.ReattachCamera` _player)
          (`/Game/Player/BP_Character.ToggleInput` _player true)
          (`/Engine/EditorBlueprintResources/StandardMacros.DoOnce` false
            (:`Completed`
              (`/Game/LevelCreation/_LevelRequirements/BP_LevelTracker.RunIntro` (`self.Level Tracker`)))))))))

(event `MoveSpawnerUp`
  (bind _player (`self.Player`))
  ;[1 1 1] Move spawner up animation
  (`Timeline|MoveSpawnerAnimation` :!via `PlayFromStart` :!label _label
    (:`Update`
      (`/Game/Game/BP_Macros.MoveComponent` (`self.Spawner`) (`self.SpawnerStartPos`) (`KismetMathLibrary.MakeVector` 0.0 0.0 (`self.MoveDistance`)) (`self.MoveSpawnerAnimation`) true
        (:`__`
          (`/Engine/EditorBlueprintResources/StandardMacros.IsValid` _player
            (:`Is Valid`
              (`/Game/Player/BP_Character.ShadowScaleOpacity` _player))))))))

(event `MoveSpawnerDown`
  ;[1 1 1] Move spawner up animation
  (goto _label :!via `Reverse`))

(fn `AttachCharacter`
  (params (Character :type "/Game/Player/BP_Character Object Reference"))
  (set `self.Player` Character)
  (`self.SetupSpawnedCharacter`))

(fn `SetupParameters`
  ;[1 1 1] Setup internal parameters
  (set `self.SpawnerStartPos` (`SceneComponent.RelativeLocation` (`self.Spawner`)))
  (bind _asbp_character (cast `/Game/Player/BP_Character` (`ChildActorComponent.ChildActor` (`self.Character`))))
  (set `self.Player` _asbp_character)
  (`self.SetupSpawnedCharacter`))

(fn `SetupSpawnedCharacter`
  (bind _player (`self.Player`))
  (`SceneComponent.K2_SetWorldTransform` (`/Game/Player/BP_Character.Camera` _player) (`SceneComponent.K2_GetComponentToWorld` (`self.CameraStartPosition`)) false false)
  (`/Game/Player/BP_Character.DetachCamera` _player)
  (`/Game/Player/BP_Character.ToggleInput` _player false))

(fn `UserConstructionScript`)