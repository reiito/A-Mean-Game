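; BP_Sign is a placeable scene sign that shows a configurable message and can optionally hover up and down.
; The construction script applies the background material to the sign mesh, and BeginPlay passes the message to the BP_SignScreen widget on the Screen component.
; When animation is enabled, a timeline lerps the sign's relative height toward a peak offset, with a FlipFlop re-triggered on finish alternating play and reverse to loop.
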(event `self.ReceiveBeginPlay`
  (`self.Initialize`)
  (`self.SetSignMessage`)
  (if (`self.Animates`)
    (`/Game/Game/BP_Macros.SetupLerpTimeline` (`self.SignAnimation`) "/Game/Data/CURVEs/CURVE_LinearLerp.CURVE_LinearLerp" (`self.AnimationSpeed`)
      (:`__`
        (`self.PlayAnimation`)))))

(event `PlayAnimation`
  (bind (_startposition_x _startposition_y _startposition_z) (`KismetMathLibrary.BreakVector` (`self.StartPosition`)))
  (`/Engine/EditorBlueprintResources/StandardMacros.FlipFlop`
    (:`A`
      (`Timeline|SignAnimation` :!label _label
        (:`Update`
          (`SceneComponent.K2_SetRelativeLocation` (`self.Sign`) (`KismetMathLibrary.MakeVector` _startposition_x _startposition_y (`KismetMathLibrary.Lerp` _startposition_z (+ _startposition_z (`self.HoveringPeakPoint`)) (`TimelineComponent.GetPlaybackPosition` (`self.SignAnimation`)))) false false))
        (:`Finished`
          (`self.PlayAnimation`))))
    (:`B`
      (goto _label :!via `Reverse`))))

(fn `Initialize`
  (bind _asbp_sign_screen (cast `/Game/LevelCreation/SceneObjects/BP_SignScreen` (`WidgetComponent.GetUserWidgetObject` (`self.Screen`))))
  (set `self.ScreenWidget` _asbp_sign_screen)
  (set `self.StartPosition` (`SceneComponent.RelativeLocation` (`self.Sign`))))

(fn `SetSignMessage`
  (`/Game/LevelCreation/SceneObjects/BP_SignScreen.SetMessage` (`self.ScreenWidget`) (`self.Message`)))

(fn `UserConstructionScript`
  (`PrimitiveComponent.SetMaterial` (`self.Sign`) 2 (`self.SignBackground`)))