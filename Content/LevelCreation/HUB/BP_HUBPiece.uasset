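; BP_HUBPiece is a modular piece of the HUB level that can be locked and unlocked.
; The construction script applies the Model and Material variables to the HUBPiece component.
; Unlock enables that component with query and physics collision, and Lock disables it.
; SetupHUBPiece reapplies only the mesh and enables the component in the same way.
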(event `self.ReceiveBeginPlay`)

(fn `Lock`
  (`/Game/Game/BP_Macros.DisableComponent` (`self.HUBPiece`)))

(fn `SetupHUBPiece`
  (`StaticMeshComponent.SetStaticMesh` (`self.HUBPiece`) (`self.Model`))
  (`/Game/Game/BP_Macros.EnableComponent` (`self.HUBPiece`) "QueryAndPhysics"))

(fn `Unlock`
  (`/Game/Game/BP_Macros.EnableComponent` (`self.HUBPiece`) "QueryAndPhysics"))

(fn `UserConstructionScript`
  (`/Game/Game/BP_Macros.SetMeshAndMaterial` (`self.HUBPiece`) (`self.Model`) (`self.Material`)))