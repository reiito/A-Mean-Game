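; Level tracker that passes level rules to the player controller and starts the level, with an optional camera intro showing the level end.
; StartLevel links and runs the PlayerSpawner, or calls RunIntro directly when none is valid.
; The intro disables input while three chained lerp timelines move the player camera to the goal, then back behind the player, blending rotation on the final leg before restoring input.
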(event `self.ReceiveBeginPlay`
  ;[1 1 1] Startup
  (`parent.ReceiveBeginPlay`)
  (`self.Initialize`)
  (`/Game/Game/BP_Macros.SetupLerpTimeline` (`self.CameraToTarget`) "/Game/Data/CURVEs/CURVE_LinearLerp.CURVE_LinearLerp" (`self.ZoomToGoalSpeed`)
    (:`__`
      (`/Game/Game/BP_Macros.SetupLerpTimeline` (`self.TargetToPlayerPhase1`) "/Game/Data/CURVEs/CURVE_LinearLerp.CURVE_LinearLerp" (`self.ZoomToPlayerSpeed`) 0.5
        (:`__`
          (`/Game/Game/BP_Macros.SetupLerpTimeline` (`self.TargetToPlayerPhase2`) "/Game/Data/CURVEs/CURVE_LinearLerp.CURVE_LinearLerp" (* (`self.ZoomToPlayerSpeed`) 2.0)
            (:`__`
              ;[1 1 1] Start Game here
              (`self.StartLevel`))))))))

(event `self.SetupReferences`
  ;[1 1 1] Extend reference setup to include player
  (`parent.SetupReferences`)
  (bind _output_get (set `self.Player` (`/Game/Player/BP_PlayerController.CurrentCharacter` (`self.PlayerController`))))
  (set `self.PlayerCamera` (`/Game/Player/BP_Character.Camera` _output_get)))

(fn `Initialize`
  (`/Game/Player/BP_PlayerController.SetLevelParams` (`self.PlayerController`) (`self.SpawnDeadBodies`) (`self.Invincible`) (`self.MaxDeadBodies`))
  (`/Game/Player/BP_PlayerController.AssignInvincibilityToPlayer` (`self.PlayerController`)))

(fn `RunIntro`
  (if (`self.PlayLevelIntro`)
    (`self.CanRunLevelIntro`
      (:`Valid`
        (`|ExecutionSequence`
          (:`then_0`
            ;[1 1 1] Setup Intro parameters
            (set `self.LevelEndPos` (`self.K2_GetActorLocation` (`self.LevelEnd`)))
            (set `self.CamStartPos` (`SceneComponent.K2_GetComponentLocation` (`self.LevelIntroStartPosition`)))
            (set `self.BehindPlayerPos` (`SceneComponent.K2_GetComponentLocation` (`/Game/Player/BP_Character.BehindTransform` (`self.Player`))))
            (set `self.InitCameraRotation` (`SceneComponent.K2_GetComponentRotation` (`self.PlayerCamera`))))
          (:`then_1`
            ;[1 1 1] Disable player input and play the intro
            (`/Game/Player/BP_Character.ToggleInput` (`self.Player`) false)
            (`TimelineComponent.Play` (`self.CameraToTarget`))))))))

(fn `StartLevel`
  (bind _playerspawner (`self.PlayerSpawner`))
  ;[1 1 1] Check for valid player spawner, assign relevant references to player controller and spawner itself
  (`/Engine/EditorBlueprintResources/StandardMacros.IsValid` _playerspawner
    (:`Is Valid`
      (set `/Game/Player/BP_PlayerController.PlayerSpawner` _playerspawner (`self.PlayerController`))
      (set `/Game/Player/BP_CharacterSpawner.Level Tracker` self _playerspawner)
      (`/Game/Player/BP_CharacterSpawner.RunBehaviour` (`self.PlayerSpawner`)))
    (:`Is Not Valid`
      (`self.RunIntro`))))

(fn `UpdateCameraToTarget`
  (`/Game/Player/BP_Character.FaceCameraLookAtPosition` (`self.Player`) (`self.LevelEndPos`))
  (`/Game/Game/BP_Macros.MoveComponent` (`self.PlayerCamera`) (`self.CamStartPos`) (+ (`self.ZoomOffset`) (`self.LevelEndPos`)) (`self.CameraToTarget`)))

(fn `UpdateTargetToPlayerPhase1`
  (locals (EndPos :type "Vector Structure"))
  (`/Game/Player/BP_Character.FaceCameraLookAtPosition` (`self.Player`) (`self.LevelEndPos`))
  (`/Game/Game/BP_Macros.MoveComponent` (`self.PlayerCamera`) (+ (`self.ZoomOffset`) (`self.LevelEndPos`)) (`self.BehindPlayerPos`) (`self.TargetToPlayerPhase1`)))

(fn `UpdateTargetToPlayerPhase2`
  (`SceneComponent.K2_SetWorldRotation` (`self.PlayerCamera`) (`KismetMathLibrary.RLerp` (`self.HalfwayRotation`) (`self.InitCameraRotation`) (`TimelineComponent.GetPlaybackPosition` (`self.TargetToPlayerPhase2`))) false false)
  (`/Game/Game/BP_Macros.MoveComponent` (`self.PlayerCamera`) (`self.HalfWayPoint`) (`self.BehindPlayerPos`) (`self.TargetToPlayerPhase2`)))

(fn `UserConstructionScript`
  (`parent.UserConstructionScript`))