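; BP_KillArea is a level-placed volume that handles actors falling into a deadly zone.
; On overlap, the player character ragdolls and is flagged as killed by the kill area.
; Falling objects return to their start position, while any other actor is destroyed.
; The construction script sizes the box from a KillAreaSize variable.
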(event `self.KillArea.OnComponentBeginOverlap`
  (params (OverlappedComponent :type "PrimitiveComponent Object Reference") (OtherActor :type "Actor Object Reference") (OtherComp :type "PrimitiveComponent Object Reference") (OtherBodyIndex :type Integer) (bFromSweep :type Boolean) (SweepResult :type "HitResult Structure (by ref)"))
  ;[1 1 1] Player
  (if (`/Game/Game/BP_Macros.IsPlayer` OtherActor)
    (bind _asbp_character (cast `/Game/Player/BP_Character` OtherActor))
    (`/Game/Player/BP_Character.Ragdoll` _asbp_character)
    (set `/Game/Player/BP_Character.DeathByKillArea` true _asbp_character)
    (else
      ;[1 1 1] Falling object
      (bind _asbp_falling_object (cast `/Game/Platforms/FallingObject/BP_FallingObject` OtherActor)
        (:`then`
          (`/Game/Platforms/FallingObject/BP_FallingObject.ReturnObjectToStart` _asbp_falling_object))
        (:`CastFailed`
          (`self.K2_DestroyActor` OtherActor) ; BP_LeftBehindObject
        )))))

(fn `UserConstructionScript`
  (`BoxComponent.SetBoxExtent` (`self.KillArea`) (`self.KillAreaSize`) true))