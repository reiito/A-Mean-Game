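; Level-end pickup that completes the current level, optionally unlocks another, saves, and opens the destination level.
; On first player hit it redirects input and plays the inherited pickup animation, with a celebration beforehand, while the obtain override handles progression through the game instance.
; A replacement mesh marks levels with a matching saved state.
; The construction script can preview that mesh in editor, and BeginPlay restores the normal mesh.
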(event `self.ReceiveBeginPlay`
  ;[1 1 1] Check if replacement mesh was set, if so reset it back
  (`|ExecutionSequence`
    (:`then_0`
      (if (`self.ViewReplacementMesh`)
        (`StaticMeshComponent.SetStaticMesh` (`self.Pickup`) (`self.PickupMesh`))))
    (:`then_1`
      (`parent.ReceiveBeginPlay`))))

(event `self.ObtainPickup`
  ;[1 1 1] Overidden functions
  ;;[1 1 1] Touch level reward, complete the level and move to level
  (`/Game/Game/BP_GameInstance.CompleteLevel` (`self.GameInstanceReference`) (`self.LevelName`))
  (`self.UnlockLevel` (`self.LevelToUnlock`))
  (`/Game/Game/BP_GameInstance.SaveEndLevel` (`self.GameInstanceReference`))
  (`GameplayStatics.OpenLevel` (`self.LevelToMoveTo`)))

(event `self.HasBeenObtained`
  ;[1 1 1] Overidden functions
  ;;[1 1 1] Check whether level has already been completed
  (bind _level_state (`/Game/Game/BP_GameInstance.GetLevelState` (`self.GameInstanceReference`) (`self.LevelName`)))
  (if (`|EnumEquality` _level_state "NewEnumerator2")
    (`self.SetReplacementMesh`)))

(event `self.BeforePickedUpAnimation`
  (`/Game/Player/BP_Character.PlayCelebrate` (`self.PlayerReference`)))

(event `self.Pickup.OnComponentHit`
  (params (HitComponent :type "PrimitiveComponent Object Reference") (OtherActor :type "Actor Object Reference") (OtherComp :type "PrimitiveComponent Object Reference") (NormalImpulse :type "Vector Structure") (Hit :type "HitResult Structure (by ref)"))
  (if (`/Game/Game/BP_Macros.IsPlayer` OtherActor)
    (bind _asbp_character (cast `/Game/Player/BP_Character` OtherActor))
    (bind _output_get (set `self.PlayerReference` _asbp_character))
    (`/Engine/EditorBlueprintResources/StandardMacros.DoOnce` false
      (:`Completed`
        (set `/Game/Player/BP_Character.InputDirectedTo` "NewEnumerator5" _output_get)
        (`self.PlayPickedUpAnimation`)))))

(fn `SetReplacementMesh`
  (`StaticMeshComponent.SetStaticMesh` (`self.Pickup`) (`self.ReplacementMesh`))
  (`PrimitiveComponent.SetMaterial` (`self.Pickup`) (`self.MaterialIndex`) (`self.ReplacementMeshMaterial`))
  (`SceneComponent.K2_SetWorldRotation` (`self.Pickup`) (`self.ReplacementMeshRotation`) false false)
  (`SceneComponent.K2_AddRelativeLocation` (`self.Pickup`) (`self.ReplacementMeshOffset`) false false))

(fn `UnlockLevel`
  (params (`Level Name` :type Name))
  (if (!= `Level Name` "None")
    (`/Game/Game/BP_GameInstance.UnlockLevel` (`self.GameInstanceReference`) `Level Name`)))

(fn `UserConstructionScript`
  (`parent.UserConstructionScript`)
  ;[1 1 1] Debug, show replacement mesh in editor
  (if (`self.ViewReplacementMesh`)
    (`self.SetReplacementMesh`)))