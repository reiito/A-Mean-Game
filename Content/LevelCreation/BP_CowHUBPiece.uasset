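; Cow piece for the HUB that can be locked or unlocked and plays a configurable idle animation.
; Construction applies the mesh and skin and derives an ID from the object name.
; SetupAnimations binds the chosen motions (hover, spin, bob, rock, stare or look away from the player) to the UpdateCowAnimation dispatcher.
; A linear timeline ping-pongs through a FlipFlop, firing that dispatcher and serving as the lerp alpha.
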(event `self.ReceiveBeginPlay`
  ;[1 1 1] Setup
  (`self.Initialize`)
  (`/Game/Game/BP_Macros.SetupLerpTimeline` (`self.CowAnimation`) "/Game/Data/CURVEs/CURVE_LinearLerp.CURVE_LinearLerp" 1.0
    (:`__`
      (`self.SetupAnimations` (`self.Parameters`)))))

(event `SetRotationAnimationUsage`
  ;[1 1 1] Animations that can be applied
  ;;[1 1 1] Rotation - Go around in circles
  (add `self.UpdateCowAnimation` (delegate `RotationAnimation`)))

(event `SetBobbingAnimationUsage`
  ;[1 1 1] Animations that can be applied
  ;;[1 1 1] Bobbing - Rotate side to side
  (`TimelineComponent.SetPlayRate` (`self.CowAnimation`) (* (`.AnimationSpeed_44_4702603543E75C7B9EE13681ED73033D` (break `/Game/LevelCreation/Pickups/STRUCT_CowCollectible` (`self.Parameters`))) 2.0))
  (add `self.UpdateCowAnimation` (delegate `BobbingAnimation`)))

(event `BobbingAnimation`
  (bind (_startrotation_roll _startrotation_pitch _startrotation_yaw) (`KismetMathLibrary.BreakRotator` (`self.StartRotation`)))
  (bind ((`BobbingAngle_45_A3BA67A94C2B7D6FDD73DD9610472793` _bobbingangle)) (break `/Game/LevelCreation/Pickups/STRUCT_CowCollectible` (`self.Parameters`)))
  ;[1 1 1] Animations that can be applied
  ;;[1 1 1] Bobbing - Rotate side to side
  (`SceneComponent.K2_SetRelativeRotation` (`self.Cow`) (`KismetMathLibrary.MakeRotator` _startrotation_roll (`KismetMathLibrary.Lerp` (* -1.0 _bobbingangle) _bobbingangle (`TimelineComponent.GetPlaybackPosition` (`self.CowAnimation`))) _startrotation_yaw) false false))

(event `RotationAnimation`
  ;[1 1 1] Animations that can be applied
  ;;[1 1 1] Rotation - Go around in circles
  (`SceneComponent.K2_AddRelativeRotation` (`self.Cow`) (`KismetMathLibrary.MakeRotator` 0.0 0.0 (`.SpinRotation_55_E794242D49941C81C62720AA7102B47C` (break `/Game/LevelCreation/Pickups/STRUCT_CowCollectible` (`self.Parameters`)))) false false))

(event `PlayCowAnimation`
  ;[1 1 1] Cow animation. Animation to use is to be binded
  (`/Engine/EditorBlueprintResources/StandardMacros.FlipFlop`
    (:`A`
      (`Timeline|CowAnimation` :!label _label
        (:`Update`
          (`self.UpdateCowAnimation`))
        (:`Finished`
          (`self.PlayCowAnimation`))))
    (:`B`
      (goto _label :!via `Reverse`))))

(event `SetHoveringAnimationUsage`
  ;[1 1 1] Animations that can be applied
  ;;[1 1 1] Hovering - Moving up then down and repeat
  (add `self.UpdateCowAnimation` (delegate `HoveringAnimation`)))

(event `SetLookingAnimationUsage`
  ;[1 1 1] Animations that can be applied
  ;;[1 1 1] Looking animation, cow faces player in some way
  (add `self.UpdateCowAnimation` (delegate `LookingAnimation`)))

(event `HoveringAnimation`
  (bind (_startposition_x _startposition_y _startposition_z) (`KismetMathLibrary.BreakVector` (`self.StartPosition`)))
  ;[1 1 1] Animations that can be applied
  ;;[1 1 1] Hovering - Moving up then down and repeat
  (`SceneComponent.K2_SetRelativeLocation` (`self.Cow`) (`KismetMathLibrary.MakeVector` _startposition_x _startposition_y (`KismetMathLibrary.Lerp` _startposition_z (+ _startposition_z (`.HoveringPeakPoint_47_89042716449BD4E3364218A45FCF73EF` (break `/Game/LevelCreation/Pickups/STRUCT_CowCollectible` (`self.Parameters`)))) (`TimelineComponent.GetPlaybackPosition` (`self.CowAnimation`)))) false false))

(event `LookingAnimation`
  (bind (_returnvalue_roll _returnvalue_pitch) (`KismetMathLibrary.BreakRotator` (`self.K2_GetActorRotation`)))
  (bind (_rotation_roll _rotation_pitch _rotation_yaw) (`KismetMathLibrary.BreakRotator` (`/Game/Game/BP_Macros.LookAtObject` (`self.Cow`) (`Character.Mesh` (`self.Player`)))))
  ;[1 1 1] Animations that can be applied
  ;;[1 1 1] Looking animation, cow faces player in some way
  (`/Engine/EditorBlueprintResources/StandardMacros.IsValid` (`self.Player`)
    (:`Is Valid`
      (`self.K2_SetActorRotation` (`KismetMathLibrary.MakeRotator` _returnvalue_roll _returnvalue_pitch _rotation_yaw)))
    (:`Is Not Valid`
      (`self.SetupPlayerReference`))))

(event `SetRockingAnimationUsage`
  ;[1 1 1] Animations that can be applied
  ;;[1 1 1] Rocking - Back and forth forward/back
  (add `self.UpdateCowAnimation` (delegate `RockingAnimation`)))

(event `RockingAnimation`
  (bind (_startrotation_roll _startrotation_pitch _startrotation_yaw) (`KismetMathLibrary.BreakRotator` (`self.StartRotation`)))
  (bind ((`RockingAngle_53_957FDC4545161579DD6FEBB75BB4C77C` _rockingangle)) (break `/Game/LevelCreation/Pickups/STRUCT_CowCollectible` (`self.Parameters`)))
  ;[1 1 1] Animations that can be applied
  ;;[1 1 1] Rocking - Back and forth forward/back
  (`SceneComponent.K2_SetRelativeRotation` (`self.Cow`) (`KismetMathLibrary.MakeRotator` (`KismetMathLibrary.Lerp` (* -1.0 _rockingangle) _rockingangle (`TimelineComponent.GetPlaybackPosition` (`self.CowAnimation`))) _startrotation_pitch _startrotation_yaw) false false))

(fn `Initialize`
  (set `self.StartPosition` (`SceneComponent.RelativeLocation` (`self.Cow`)))
  (set `self.StartRotation` (`SceneComponent.RelativeRotation` (`self.Cow`))))

(fn `Lock`
  (`/Game/Game/BP_Macros.DisableComponent` (`self.Cow`)))

(fn `SetupAnimations`
  (params (Params :type "/Game/LevelCreation/Pickups/STRUCT_CowCollectible Structure"))
  (bind _cow (`self.Cow`))
  (`|ExecutionSequence`
    (:`then_0`
      (bind _output_get (set `self.Parameters` Params))
      (bind ((`AnimationToPlay_46_7FB849DF49D33EA5E928B7A133914EF5` _animationtoplay) (`AnimationSpeed_44_4702603543E75C7B9EE13681ED73033D` _animationspeed)) (break `/Game/LevelCreation/Pickups/STRUCT_CowCollectible` _output_get))
      (`/Game/Game/BP_Macros.SetupLerpTimeline` (`self.CowAnimation`) "/Game/Data/CURVEs/CURVE_LinearLerp.CURVE_LinearLerp" _animationspeed
        (:`__`
          (switch `/Game/LevelCreation/Pickups/ENUM_PickupAnimationType` _animationtoplay
            (:`NewEnumerator3`
              (`self.SetHoveringAnimationUsage`))
            (:`NewEnumerator4`
              (`self.SetRotationAnimationUsage`))
            (:`NewEnumerator0`
              (`self.SetHoveringAnimationUsage`)
              (`self.SetRotationAnimationUsage`))
            (:`NewEnumerator1`
              (`self.SetBobbingAnimationUsage`))
            (:`NewEnumerator5`
              (`SceneComponent.K2_SetRelativeRotation` _cow (struct :`Yaw` 90.0) false false)
              (`self.SetupPlayerReference` :!label _label)
              (`self.SetLookingAnimationUsage`))
            (:`NewEnumerator6`
              (`SceneComponent.K2_SetRelativeRotation` _cow (struct :`Yaw` -90.0) false false)
              (goto _label))
            (:`NewEnumerator7`
              (`self.SetRockingAnimationUsage`))))))
    (:`then_1`
      (`self.PlayCowAnimation`))))

(fn `SetupPlayerReference`
  (bind _asbp_player_controller (cast `/Game/Player/BP_PlayerController` (`GameplayStatics.GetPlayerController` 0)))
  (set `self.Player` (`/Game/Player/BP_PlayerController.CurrentCharacter` _asbp_player_controller)))

(fn `Unlock`
  (`/Game/Game/BP_Macros.EnableComponent` (`self.Cow`) "QueryAndPhysics"))

(fn `UserConstructionScript`
  (`/Game/Game/BP_Macros.SetMeshAndMaterial` (`self.Cow`) (`self.CowModel`) (`self.CowSkin`)
    (:`__`
      (set `self.ID` (`KismetStringLibrary.Conv_StringToName` (`KismetSystemLibrary.GetObjectName` self))))))