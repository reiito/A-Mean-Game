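; BP_CameraShifter is a placeable trigger volume that turns the player's camera to a set facing when the player enters it.
; The construction script sizes and offsets the overlap box and orients a Direction component from the Facing setting.
; On overlap it disables camera input and runs a timeline that lerps control rotation to Direction's world yaw along the shortest path, keeping pitch and roll, then re-enables input.
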(event `self.ReceiveBeginPlay`
  (bind _asbp_player_controller (cast `/Game/Player/BP_PlayerController` (`GameplayStatics.GetPlayerController` 0)))
  (set `self.PlayerController` _asbp_player_controller)
  (`/Game/Game/BP_Macros.SetupLerpTimeline` (`self.Animation`) "/Game/Data/CURVEs/CURVE_LinearLerp.CURVE_LinearLerp" (`self.AnimationSpeed`)))

(event `self.OverlapArea.OnComponentBeginOverlap`
  (params (OverlappedComponent :type "PrimitiveComponent Object Reference") (OtherActor :type "Actor Object Reference") (OtherComp :type "PrimitiveComponent Object Reference") (OtherBodyIndex :type Integer) (bFromSweep :type Boolean) (SweepResult :type "HitResult Structure (by ref)"))
  (if (`/Game/Game/BP_Macros.IsPlayer` OtherActor)
    (bind _asbp_character (cast `/Game/Player/BP_Character` OtherActor))
    (set `self.Player` _asbp_character)
    (`self.RotateCamera`)))

(event `RotateCamera`
  (bind (_playerrotation_roll _playerrotation_pitch _playerrotation_yaw) (`KismetMathLibrary.BreakRotator` (`self.PlayerRotation`)))
  (bind (_returnvalue_roll _returnvalue_pitch _returnvalue_yaw) (`KismetMathLibrary.BreakRotator` (`SceneComponent.K2_GetComponentRotation` (`self.Direction`))))
  ;[1 1 1] Rotate from z axis to face direction
  (`self.GetRotations`)
  (`Timeline|Animation` :!via `PlayFromStart`
    (:`Update`
      (`Controller.SetControlRotation` (`self.PlayerController`) (`KismetMathLibrary.RLerp` (`KismetMathLibrary.MakeRotator` _playerrotation_roll _playerrotation_pitch _playerrotation_yaw) (`KismetMathLibrary.MakeRotator` _playerrotation_roll _playerrotation_pitch _returnvalue_yaw) (`TimelineComponent.GetPlaybackPosition` (`self.Animation`)) true)))
    (:`Finished`
      (set `/Game/Player/BP_Character.CameraInputEnabled` true (`self.Player`)))))

(fn `GetRotations`
  (set `self.PlayerRotation` (`Controller.GetControlRotation` (`self.PlayerController`)))
  (set `self.FixedRotation` (`SceneComponent.RelativeRotation` (`self.Direction`)))
  (set `/Game/Player/BP_Character.CameraInputEnabled` false (`self.Player`)))

(fn `SetFacingDirection`
  (switch `/Game/Data/ENUMs/ENUM_Direction` (`self.Facing`)
    (:`NewEnumerator0`
      (`SceneComponent.K2_SetRelativeRotation` (`self.Direction`) (struct :`Pitch` 90.0) false false))
    (:`NewEnumerator1`
      (`SceneComponent.K2_SetRelativeRotation` (`self.Direction`) (struct :`Pitch` -90.0) false false))
    (:`NewEnumerator2`
      (`SceneComponent.K2_SetRelativeRotation` (`self.Direction`) (struct :`Yaw` -90.0) false false))
    (:`NewEnumerator3`
      (`SceneComponent.K2_SetRelativeRotation` (`self.Direction`) (struct :`Yaw` 90.0) false false))
    (:`NewEnumerator5`
      (`SceneComponent.K2_SetRelativeRotation` (`self.Direction`) (struct :`Yaw` 180.0) false false))))

(fn `UserConstructionScript`
  (bind (_size_x _size_y _size_z) (`KismetMathLibrary.BreakVector` (`self.Size`)))
  (bind (_size_x_2 _size_y_2 _size_z_2) (`KismetMathLibrary.BreakVector` (`self.Size`)))
  (`SceneComponent.K2_AddRelativeLocation` (`self.OverlapArea`) (`KismetMathLibrary.MakeVector` _size_x 0.0 _size_z) false false)
  (`SceneComponent.K2_AddRelativeLocation` (`self.Direction`) (`KismetMathLibrary.MakeVector` _size_x_2 0.0 (* _size_z_2 2.0)) false false)
  (`BoxComponent.SetBoxExtent` (`self.OverlapArea`) (`self.Size`) true)
  (`self.SetFacingDirection`))