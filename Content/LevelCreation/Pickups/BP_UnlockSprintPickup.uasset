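; Pickup that permanently unlocks the sprint ability for the player, extending a parent pickup's startup and collection logic.
; On collection it saves the unlock through the game instance, has the player controller reassign unlockables, notifies the game mode and destroys itself.
; A macro checks the game instance at BeginPlay to disable the pickup if sprint is already unlocked.
; An overridden animation update spins and ease-scales the pickup mesh.
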(event `self.ReceiveBeginPlay`
  ;[1 1 1] Startup
  (`parent.ReceiveBeginPlay`)
  (`self.HasSprintBeenObtained`
    (:`Obtained`
      (`/Game/Game/BP_Macros.DisableComponent` (`self.Pickup`)))))

(event `self.ObtainPickup`
  (bind _gameinstancereference (`self.GameInstanceReference`))
  ;[1 1 1] Obtain pickup, unlock sprint in player
  (`parent.ObtainPickup`)
  (`/Game/Game/BP_GameInstance.UnlockSprint` _gameinstancereference)
  (`/Game/Game/BP_GameInstance.SaveSprint` _gameinstancereference)
  (bind _asbp_player_controller (cast `/Game/Player/BP_PlayerController` (`GameplayStatics.GetPlayerController` 0)))
  (`/Game/Player/BP_PlayerController.AssignUnlockablesToPlayer` _asbp_player_controller true)
  (`/Game/Game/BP_GameMode.SprintObtained` (`self.GameMode`))
  (`self.K2_DestroyActor`))

(event `self.UpdatePickedUpAnimation`
  (bind _pickup (`self.Pickup`))
  (`SceneComponent.K2_AddRelativeRotation` _pickup (`KismetMathLibrary.MakeRotator` 0.0 0.0 (`self.PickedUpSpinSpeed`)) false false)
  (`SceneComponent.SetWorldScale3D` _pickup (`|EaseFunction` "EaseInOut" (`TimelineComponent.GetPlaybackPosition` (`self.PickedUpAnimation`)) (`self.PickupSize`))))

(fn `UserConstructionScript`
  (`parent.UserConstructionScript`))