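; Pickup that permanently unlocks the player's double jump, built on a parent pickup class.
; On BeginPlay it disables its pickup component if the GameInstance says double jump is already unlocked.
; When obtained, it sets and saves the unlock in the GameInstance, has the player controller reapply unlockables, notifies the GameMode and destroys itself.
; An animation update event spins and eases the pickup's scale using the picked-up timeline's position.
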(event `self.ReceiveBeginPlay`
  ;[1 1 1] Startup
  (`parent.ReceiveBeginPlay`)
  (`self.HasDoubleJumpBeenObtained`
    (:`Obtained`
      (`/Game/Game/BP_Macros.DisableComponent` (`self.Pickup`)))))

(event `self.ObtainPickup`
  (bind _gameinstancereference (`self.GameInstanceReference`))
  ;[1 1 1] Obtain pickup, enable double jump for player
  (`parent.ObtainPickup`)
  (`/Game/Game/BP_GameInstance.UnlockDoubleJump` _gameinstancereference)
  (`/Game/Game/BP_GameInstance.SaveDoubleJump` _gameinstancereference)
  (bind _asbp_player_controller (cast `/Game/Player/BP_PlayerController` (`GameplayStatics.GetPlayerController` 0)))
  (`/Game/Player/BP_PlayerController.AssignUnlockablesToPlayer` _asbp_player_controller true)
  (`/Game/Game/BP_GameMode.DoubleJumpObtained` (`self.GameMode`))
  (`self.K2_DestroyActor`))

(event `self.UpdatePickedUpAnimation`
  (bind _pickup (`self.Pickup`))
  (`SceneComponent.K2_AddRelativeRotation` _pickup (`KismetMathLibrary.MakeRotator` 0.0 0.0 (`self.PickedUpSpinSpeed`)) false false)
  (`SceneComponent.SetWorldScale3D` _pickup (`|EaseFunction` "Linear" (`TimelineComponent.GetPlaybackPosition` (`self.PickedUpAnimation`)) (`self.PickupSize`))))

(fn `UserConstructionScript`
  (`parent.UserConstructionScript`))