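; BP_UnlockablePickup is an unlockable pickup that spins and hovers while idle.
; On BeginPlay it runs the parent logic, then casts and caches BP_GameMode.
; The IdleAnimation timeline update adds a yaw rotation to the Pickup component and lerps its height between StartPosition and HoveringPeakPoint above it, using the timeline's playback position as alpha.
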(event `self.ReceiveBeginPlay`
  (`parent.ReceiveBeginPlay`)
  (bind _asbp_game_mode (cast `/Game/Game/BP_GameMode` (`GameplayStatics.GetGameMode`)))
  (set `self.GameMode` _asbp_game_mode))

(event `self.IdleAnimation__UpdateFunc`
  (bind (_startposition_x _startposition_y _startposition_z) (`KismetMathLibrary.BreakVector` (`self.StartPosition`)))
  ;[1 1 1] Spin around in circles
  (`SceneComponent.K2_AddRelativeRotation` (`self.Pickup`) (`KismetMathLibrary.MakeRotator` 0.0 0.0 (`self.SpinRotation`)) false false)
  ;[1 1 1] Hover up and down
  (`SceneComponent.K2_SetRelativeLocation` (`self.Pickup`) (`KismetMathLibrary.MakeVector` _startposition_x _startposition_y (`KismetMathLibrary.Lerp` _startposition_z (+ _startposition_z (`self.HoveringPeakPoint`)) (`TimelineComponent.GetPlaybackPosition` (`self.IdleAnimation`)))) false false))

(fn `UserConstructionScript`
  (`parent.UserConstructionScript`))