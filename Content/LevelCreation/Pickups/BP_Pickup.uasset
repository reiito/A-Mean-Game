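; BP_Pickup is a base pickup actor with an optional platform, built from configurable meshes, materials and transforms.
; Timelines drive a back-and-forth idle animation and a one-shot pickup animation, triggered by player overlap, that destroys the pickup component and calls ObtainPickup.
; ObtainPickup updates the player's spawn point for checkpoints, while empty functions leave obtained-state, reset and animation behaviour to children.
; A separate box trigger disables the player's jump while overlapped.
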(event `self.ReceiveBeginPlay`
  ;[1 1 1] Startup
  (`/Game/Game/BP_Macros.SetupLerpTimeline` (`self.IdleAnimation`) "/Game/Data/CURVEs/CURVE_LinearLerp.CURVE_LinearLerp" (`self.IdleAnimSpeed`)
    (:`__`
      (`/Game/Game/BP_Macros.SetupLerpTimeline` (`self.PickedUpAnimation`) "/Game/Data/CURVEs/CURVE_LinearLerp.CURVE_LinearLerp" (`self.PickedUpAnimSpeed`)
        (:`__`
          (`self.SetupReferences`)
          (`self.HasBeenObtained`)
          (`self.PlayIdleAnimation`))))))

(event `PlayIdleAnimation`
  ;[1 1 1] Animation
  (`/Engine/EditorBlueprintResources/StandardMacros.FlipFlop`
    (:`A`
      (`Timeline|IdleAnimation` :!label _label
        (:`Update`
          (`self.UpdateIdleAnimation`))
        (:`Finished`
          (`self.PlayIdleAnimation`))))
    (:`B`
      (goto _label :!via `Reverse`))))

(event `self.Pickup.OnComponentBeginOverlap`
  (params (OverlappedComponent :type "PrimitiveComponent Object Reference") (OtherActor :type "Actor Object Reference") (OtherComp :type "PrimitiveComponent Object Reference") (OtherBodyIndex :type Integer) (bFromSweep :type Boolean) (SweepResult :type "HitResult Structure (by ref)"))
  ;[1 1 1] Pickup, destroy component and run obtain function (to be implemented in child
  (if (`/Game/Game/BP_Macros.IsPlayer` OtherActor)
    (bind _asbp_character (cast `/Game/Player/BP_Character` OtherActor))
    (set `self.PlayerReference` _asbp_character)
    (`TimelineComponent.Stop` (`self.IdleAnimation`))
    (`self.PlayPickedUpAnimation`)))

(event `self.DisableJumpTrigger.OnComponentBeginOverlap`
  (params (OverlappedComponent :type "PrimitiveComponent Object Reference") (OtherActor :type "Actor Object Reference") (OtherComp :type "PrimitiveComponent Object Reference") (OtherBodyIndex :type Integer) (bFromSweep :type Boolean) (SweepResult :type "HitResult Structure (by ref)"))
  (if (`/Game/Game/BP_Macros.IsPlayer` OtherActor)
    (bind _asbp_character (cast `/Game/Player/BP_Character` OtherActor))
    (set `/Game/Player/BP_Character.JumpEnabled` false _asbp_character)))

(event `self.K2_OnReset`
  ;[1 1 1] Reset, player respawned
  (`self.ResetPickup`))

(event `self.DisableJumpTrigger.OnComponentEndOverlap`
  (params (OverlappedComponent :type "PrimitiveComponent Object Reference") (OtherActor :type "Actor Object Reference") (OtherComp :type "PrimitiveComponent Object Reference") (OtherBodyIndex :type Integer))
  (if (`/Game/Game/BP_Macros.IsPlayer` OtherActor)
    (bind _asbp_character (cast `/Game/Player/BP_Character` OtherActor))
    (set `/Game/Player/BP_Character.JumpEnabled` true _asbp_character)))

(event `PlayPickedUpAnimation`
  (`/Engine/EditorBlueprintResources/StandardMacros.DoOnce` false
    (:`Completed`
      (`self.BeforePickedUpAnimation`)
      (`Timeline|PickedUpAnimation` :!via `PlayFromStart`
        (:`Update`
          (`self.UpdatePickedUpAnimation`))
        (:`Finished`
          (`ActorComponent.K2_DestroyComponent` (`self.Pickup`))
          (`self.ObtainPickup`))))))

(fn `BeforePickedUpAnimation`)

(fn `HasBeenObtained`)

(fn `ObtainPickup`
  (if (`self.Checkpoint`)
    (bind _asbp_player_controller (cast `/Game/Player/BP_PlayerController` (`GameplayStatics.GetPlayerController` 0)))
    (set `/Game/Player/BP_PlayerController.PlayerSpawnPoint` (`SceneComponent.K2_GetComponentToWorld` (`self.DefaultSceneRoot`)) _asbp_player_controller)))

(fn `ResetPickup`)

(fn `SetupPickup`
  (`/Game/Game/BP_Macros.SetMeshAndMaterial` (`self.Platform`) (`self.PlatformMesh`) (`self.PlatformMaterial`)
    (:`__`
      (`/Game/Game/BP_Macros.SetMeshAndMaterial` (`self.Pickup`) (`self.PickupMesh`) (`self.PickupMaterial`)
        (:`__`
          (`SceneComponent.SetRelativeScale3D` (`self.Pickup`) (`self.PickupSize`))
          (`SceneComponent.K2_AddRelativeLocation` (`self.Pickup`) (`self.StartPosition`) false false)
          (`SceneComponent.K2_SetRelativeRotation` (`self.Pickup`) (`self.StartRotation`) false false))))))

(fn `SetupReferences`
  (bind _asbp_game_instance (cast `/Game/Game/BP_GameInstance` (`GameplayStatics.GetGameInstance`)))
  (set `self.GameInstanceReference` _asbp_game_instance))

(fn `UpdatePickedUpAnimation`)

(fn `UserConstructionScript`
  (`BoxComponent.SetBoxExtent` (`self.DisableJumpTrigger`) (`self.DisableJumpTriggerSize`) true)
  (`SceneComponent.K2_AddLocalOffset` (`self.DisableJumpTrigger`) (`self.DisableJumpTriggerOffset`) false false)
  (`self.SetupPickup`)
  (bind _returnvalue (`GameplayStatics.GetCurrentLevelName` true))
  (set `self.LevelName` (`KismetStringLibrary.Conv_StringToName` _returnvalue))
  (if (not (`self.HasPlatform`))
    (`/Game/Game/BP_Macros.DisableComponent` (`self.Platform`))))