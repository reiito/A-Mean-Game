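; Cow collectible pickup that reports to the game mode when obtained and saves itself to the game instance under an ID taken from its object name.
; On BeginPlay, already-obtained cows disable their mesh; others set custom depth from the CowsVisible flag and bind their chosen idle animation.
; Idle options include hovering, spinning, bobbing, rocking and facing toward or away from the player, mostly lerped over the IdleAnimation timeline.
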(event `SetupAnimations`
  ;[1 1 1] Determine animation to use
  (switch `/Game/LevelCreation/Pickups/ENUM_PickupAnimationType` (`self.AnimationToPlay`)
    (:`NewEnumerator3`
      (`self.SetHoveringAnimationUsage`))
    (:`NewEnumerator4`
      (`self.SetRotationAnimationUsage`))
    (:`NewEnumerator0`
      (`self.SetHoveringAnimationUsage`)
      (`self.SetRotationAnimationUsage`))
    (:`NewEnumerator1`
      (`self.SetBobbingAnimationUsage`))
    (:`NewEnumerator5`
      (`SceneComponent.K2_SetRelativeRotation` (`self.Pickup`) (struct :`Yaw` 90.0) false false)
      (`self.SetupPlayerReference` :!label _label)
      (`self.SetLookingAnimationUsage`))
    (:`NewEnumerator6`
      (`SceneComponent.K2_SetRelativeRotation` (`self.Pickup`) (struct :`Yaw` -90.0) false false)
      (goto _label))
    (:`NewEnumerator7`
      (`self.SetRockingAnimationUsage`))))

(event `self.ReceiveBeginPlay`
  ;[1 1 1] Startup - Setup animations only when obtained
  (`parent.ReceiveBeginPlay`)
  (`self.BeenObtained`
    (:`Obtained`
      (`/Game/Game/BP_Macros.DisableComponent` (`self.Pickup`)))
    (:`NotYetObtained`
      (`self.Initialize`))))

(event `self.ObtainPickup`
  ;[1 1 1] Pickup collectible
  (`/Game/Game/BP_GameMode.CowObtained` (`self.GameMode`) (`self.ObtainPopupTexture`) (`self.ObtainPopupMessage`))
  (`/Game/Game/BP_GameInstance.ObtainCow` (`self.GameInstanceReference`) (`self.ID`) (`self.StoreParameters`)))

(event `SetRotationAnimationUsage`
  ;[1 1 1] Animations that can be applied
  ;;[1 1 1] Rotation - Go around in circles
  (add `self.UpdateIdleAnimation` (delegate `RotationAnimation`)))

(event `SetBobbingAnimationUsage`
  ;[1 1 1] Animations that can be applied
  ;;[1 1 1] Bobbing - Rotate side to side
  (`TimelineComponent.SetPlayRate` (`self.IdleAnimation`) (* (`self.IdleAnimSpeed`) 2.0))
  (add `self.UpdateIdleAnimation` (delegate `BobbingAnimation`)))

(event `BobbingAnimation`
  (bind _bobbingangle (`self.BobbingAngle`))
  (bind (_startrotation_roll _startrotation_pitch _startrotation_yaw) (`KismetMathLibrary.BreakRotator` (`self.StartRotation`)))
  ;[1 1 1] Animations that can be applied
  ;;[1 1 1] Bobbing - Rotate side to side
  (`SceneComponent.K2_SetRelativeRotation` (`self.Pickup`) (`KismetMathLibrary.MakeRotator` _startrotation_roll (`KismetMathLibrary.Lerp` (* -1.0 _bobbingangle) _bobbingangle (`TimelineComponent.GetPlaybackPosition` (`self.IdleAnimation`))) _startrotation_yaw) false false))

(event `RotationAnimation`
  ;[1 1 1] Animations that can be applied
  ;;[1 1 1] Rotation - Go around in circles
  (`SceneComponent.K2_AddRelativeRotation` (`self.Pickup`) (`KismetMathLibrary.MakeRotator` 0.0 0.0 (`self.SpinRotation`)) false false))

(event `SetHoveringAnimationUsage`
  ;[1 1 1] Animations that can be applied
  ;;[1 1 1] Hovering - Moving up then down and repeat
  (add `self.UpdateIdleAnimation` (delegate `HoveringAnimation`)))

(event `SetLookingAnimationUsage`
  ;[1 1 1] Animations that can be applied
  ;;[1 1 1] Looking animation, cow faces player in some way
  (add `self.UpdateIdleAnimation` (delegate `LookingAnimation`)))

(event `HoveringAnimation`
  (bind (_startposition_x _startposition_y _startposition_z) (`KismetMathLibrary.BreakVector` (`self.StartPosition`)))
  ;[1 1 1] Animations that can be applied
  ;;[1 1 1] Hovering - Moving up then down and repeat
  (`SceneComponent.K2_SetRelativeLocation` (`self.Pickup`) (`KismetMathLibrary.MakeVector` _startposition_x _startposition_y (`KismetMathLibrary.Lerp` _startposition_z (+ _startposition_z (`self.HoveringPeakPoint`)) (`TimelineComponent.GetPlaybackPosition` (`self.IdleAnimation`)))) false false))

(event `LookingAnimation`
  (bind (_returnvalue_roll _returnvalue_pitch) (`KismetMathLibrary.BreakRotator` (`self.K2_GetActorRotation`)))
  (bind (_rotation_roll _rotation_pitch _rotation_yaw) (`KismetMathLibrary.BreakRotator` (`/Game/Game/BP_Macros.LookAtObject` (`self.Pickup`) (`Character.Mesh` (`self.Character`)))))
  ;[1 1 1] Animations that can be applied
  ;;[1 1 1] Looking animation, cow faces player in some way
  (`/Engine/EditorBlueprintResources/StandardMacros.IsValid` (`self.Character`)
    (:`Is Valid`
      (`self.K2_SetActorRotation` (`KismetMathLibrary.MakeRotator` _returnvalue_roll _returnvalue_pitch _rotation_yaw)))
    (:`Is Not Valid`
      (`self.SetupPlayerReference`))))

(event `SetRockingAnimationUsage`
  ;[1 1 1] Animations that can be applied
  ;;[1 1 1] Rocking - Back and forth forward/back
  (add `self.UpdateIdleAnimation` (delegate `RockingAnimation`)))

(event `RockingAnimation`
  (bind (_startrotation_roll _startrotation_pitch _startrotation_yaw) (`KismetMathLibrary.BreakRotator` (`self.StartRotation`)))
  (bind _rockingangle (`self.RockingAngle`))
  ;[1 1 1] Animations that can be applied
  ;;[1 1 1] Rocking - Back and forth forward/back
  (`SceneComponent.K2_SetRelativeRotation` (`self.Pickup`) (`KismetMathLibrary.MakeRotator` (`KismetMathLibrary.Lerp` (* -1.0 _rockingangle) _rockingangle (`TimelineComponent.GetPlaybackPosition` (`self.IdleAnimation`))) _startrotation_pitch _startrotation_yaw) false false))

(event `self.UpdatePickedUpAnimation`
  ;[1 1 1] Animations that can be applied
  (`SceneComponent.SetWorldScale3D` (`self.Pickup`) (`|EaseFunction` "EaseInOut" (`TimelineComponent.GetPlaybackPosition` (`self.PickedUpAnimation`)) (`self.PickupSize`))))

(fn `Initialize`
  (bind _asbp_game_mode (cast `/Game/Game/BP_GameMode` (`GameplayStatics.GetGameMode`)))
  (set `self.GameMode` _asbp_game_mode)
  (`self.SetupAnimations`)
  (`self.SetVisible`))

(fn `ResetParameters`
  (returns (STRUCT_CowCollectible :type "/Game/LevelCreation/Pickups/STRUCT_CowCollectible Structure"))
  (return (make `/Game/LevelCreation/Pickups/STRUCT_CowCollectible` false (`self.AnimationToPlay`) (`self.HoveringPeakPoint`) (`self.BobbingAngle`) (`self.RockingAngle`) (`self.SpinRotation`) (`self.IdleAnimSpeed`))))

(fn `SetupPlayerReference`
  (bind _asbp_character (cast `/Game/Player/BP_Character` (`GameplayStatics.GetPlayerPawn` 0)))
  (set `self.Character` _asbp_character))

(fn `SetVisible`
  (bind _pickup (`self.Pickup`))
  (if (`/Game/Game/BP_GameInstance.CowsVisible` (`self.GameInstanceReference`))
    (`PrimitiveComponent.SetRenderCustomDepth` _pickup true)
    (else
      (`PrimitiveComponent.SetRenderCustomDepth` _pickup false))))

(fn `UserConstructionScript`
  (`parent.UserConstructionScript`)
  ;[1 1 1] Assign ID
  (set `self.ID` (`KismetStringLibrary.Conv_StringToName` (`KismetSystemLibrary.GetObjectName` self))))