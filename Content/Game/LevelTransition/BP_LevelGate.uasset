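; Level gate actor for level transitions, with a collapsible barrier and labels showing level, furniture and cow status.
; The construction script applies configurable meshes, sizes and side-label layout, then blanks the labels.
; UnlockGate and LockGate play or reverse a timeline intended to scale the barrier pivot's Z between full and zero.
; Its finish logic either reveals icons from the stored level state and cow flag or resets them to blank.
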(event `self.ReceiveBeginPlay`
  (`/Game/Game/BP_Macros.SetupLerpTimeline` (`self.UnlockAnimation`) "/Game/Data/CURVEs/CURVE_LinearLerp.CURVE_LinearLerp" (`self.AnimationSpeed`)
    (:`__`
      (`PrimitiveComponent.SetMaterial` (`self.LevelLabel`) 2 (`self.BlankLabel`)))))

(fn `LockGate`
  (`TimelineComponent.Reverse` (`self.UnlockAnimation`)))

(fn `SetCowLabelState`
  (set `self.CowObtained` true))

(fn `SetFurnitureLabelState`
  (params (State :type "/Game/Game/LevelTransition/ENUM_LevelState Enum" :default "NewEnumerator0"))
  (set `self.LevelState` State))

(fn `SetupLabelDefaults`
  (bind _blanklabel (`self.BlankLabel`))
  (`PrimitiveComponent.SetMaterial` (`self.LevelLabel`) 2 _blanklabel)
  (`PrimitiveComponent.SetMaterial` (`self.FurnitureLabel`) 2 _blanklabel)
  (`PrimitiveComponent.SetMaterial` (`self.CowLabel`) 2 _blanklabel))

(fn `SetupLabelPositions`
  (params (Postion :type "/Game/Data/ENUMs/ENUM_SignPosition Enum" :default "NewEnumerator0"))
  (bind _furniturelabel (`self.FurnitureLabel`))
  (bind _cowlabel (`self.CowLabel`))
  (bind _labeloffset (`self.LabelOffset`))
  (bind _relativelocation (`SceneComponent.RelativeLocation` (`self.LeftTop`)))
  (bind _relativelocation_2 (`SceneComponent.RelativeLocation` (`self.RightTop`)))
  (switch `/Game/Data/ENUMs/ENUM_SignPosition` Postion
    (:`NewEnumerator0`
      (`SceneComponent.K2_SetRelativeLocation` _furniturelabel _relativelocation false false)
      (`SceneComponent.K2_SetRelativeLocation` _cowlabel _relativelocation_2 false false))
    (:`NewEnumerator1`
      (`SceneComponent.K2_SetRelativeLocation` _furniturelabel _relativelocation false false)
      (`SceneComponent.K2_SetRelativeLocation` _cowlabel (`SceneComponent.RelativeLocation` (`self.LeftBot`)) false false))
    (:`NewEnumerator2`
      (`SceneComponent.K2_SetRelativeLocation` _furniturelabel _relativelocation_2 false false)
      (`SceneComponent.K2_SetRelativeLocation` _cowlabel (`SceneComponent.RelativeLocation` (`self.RightBot`)) false false)))
  (`SceneComponent.K2_AddRelativeLocation` _furniturelabel (`KismetMathLibrary.MakeVector` _labeloffset) false false)
  (`SceneComponent.K2_AddRelativeLocation` _cowlabel (`KismetMathLibrary.MakeVector` _labeloffset) false false))

(fn `ToggleSideLabelsVisibility`
  (switch `/Game/Game/LevelTransition/ENUM_LevelState` (`self.LevelState`)
    (:`NewEnumerator1`
      ;[1 1 1] Level unlocked, show locked icons
      (`PrimitiveComponent.SetMaterial` (`self.CowLabel`) 2 (`self.LockedCowLabel`))
      (`PrimitiveComponent.SetMaterial` (`self.FurnitureLabel`) 2 (`self.LockedFurnitureLabel`)))
    (:`NewEnumerator2`
      ;[1 1 1] Level complete, show furniture icon, determine whether cow obtained
      (`PrimitiveComponent.SetMaterial` (`self.FurnitureLabel`) 2 (`self.ObtainedFurnitureLabel`))
      (if (`self.CowObtained`)
        (`PrimitiveComponent.SetMaterial` (`self.CowLabel`) 2 (`self.ObtainedCowLabel`))
        (else
          (`PrimitiveComponent.SetMaterial` (`self.CowLabel`) 2 (`self.LockedCowLabel`)))))))

(fn `UnlockGate`
  (`TimelineComponent.Play` (`self.UnlockAnimation`)))

(fn `UpdateBarrierAnimation`
  (`SceneComponent.SetRelativeScale3D` (`self.BarrierPivot`) (`KismetMathLibrary.VLerp` (1.0 1.0 1.0) (1.0 1.0 0.0) (`TimelineComponent.GetPlaybackPosition` (`self.UnlockAnimation`)))))

(fn `UserConstructionScript`
  (bind _levellabel (`self.LevelLabel`))
  (`StaticMeshComponent.SetStaticMesh` (`self.Top`) (`self.GateTopModel`))
  (`StaticMeshComponent.SetStaticMesh` (`self.Barrier`) (`self.GateBarrierModel`))
  (`SceneComponent.SetRelativeScale3D` _levellabel (`self.LabelSize`))
  (`SceneComponent.K2_AddRelativeLocation` _levellabel (`KismetMathLibrary.MakeVector` (`self.LabelOffset`)) false false)
  (`SceneComponent.SetRelativeScale3D` (`self.Gate`) (`self.GateSize`))
  (`self.SetupLabelPositions` (`self.Positions`))
  (`self.SetupLabelDefaults`))