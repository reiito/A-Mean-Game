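; BP_HUBTracker manages the hub's level progression, setting up gates, hub pieces and collectible cows from GameInstance state.
; On BeginPlay it locks or unlocks each Levels entry, with override flags for showcase unlocking and cow data.
; Unlocked levels bind their transition platform's hit event, and a platform-to-index map picks the level to open, optionally through a GameMode loading-screen transition.
; It also shows the end screen once after game completion.
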(event `self.ReceiveBeginPlay`
  ;[1 1 1] Setup
  (`parent.ReceiveBeginPlay`)
  (`self.SetupLevels`)
  (`self.CheckGameComplete`))

(event `AddLevelTransition`
  (params (LevelParams :type "/Game/Game/LevelTransition/STRUCT_LevelTransitionParameters Structure (by ref)"))
  ;[1 1 1] Set trap to transport player to level
  (add `/Game/Platforms/BP_Killable.HitPlayer` (`.LevelTransitionPlatform_25_F3C83AF7499F67344C459C905D6240B8` (break `/Game/Game/LevelTransition/STRUCT_LevelTransitionParameters` LevelParams)) (delegate `TransitionToLevel`)))

(event `TransitionToLevel`
  (params (HitBy :type "/Game/Platforms/BP_Killable Object Reference"))
  (bind ((`LevelName_24_50A6B0C84C53A264E6DBD4BF8EF57C39` _levelname) (`ChanceForRandomCharacter_30_8411E9AD4AE070837F02EA97A62E5BE0` _chanceforrandomcharacter)) (break `/Game/Game/LevelTransition/STRUCT_LevelTransitionParameters` (`|GetArrayItem` (`self.Levels`) (`BlueprintMapLibrary.Map_Find` (`self.Transitions`) HitBy))))
  ;[1 1 1] Set trap to transport player to level
  (if (`self.RunLoadingScreen`)
    (`KismetSystemLibrary.Delay` (`self.LoadingScreenDelay`))
    (`/Game/Game/BP_GameMode.RunLevelTransition` (`self.GameMode`) _chanceforrandomcharacter _levelname)
    (else
      (`GameplayStatics.OpenLevel` _levelname))))

(fn `CheckGameComplete`
  (bind _gameinstance (`self.GameInstance`))
  (bind _gamemode (`self.GameMode`))
  (if (and (`/Game/Game/BP_GameInstance.GameCompleted` _gameinstance) (not (`/Game/Game/BP_GameInstance.EndShown` _gameinstance)))
    (`/Game/Game/BP_UI.ViewEndScreen` (`/Game/Game/BP_GameMode.HUDWidget` _gamemode))
    (set `/Game/Player/BP_Character.InputDirectedTo` "NewEnumerator6" (`/Game/Game/BP_GameMode.Player` _gamemode))
    (`/Game/Game/BP_GameInstance.SaveEndShown` _gameinstance)))

(fn `LockLevel`
  (params (Level :type "/Game/Game/LevelTransition/STRUCT_LevelTransitionParameters Structure"))
  (`/Game/Game/LevelTransition/BP_LevelGate.LockGate` (`.LevelGate_33_37F0881240130F38A98BDEBF03AA7C9F` (break `/Game/Game/LevelTransition/STRUCT_LevelTransitionParameters` Level))))

(fn `SetupCow`
  (params (Obtained :type Boolean) (Cow :type "/Game/LevelCreation/BP_CowHUBPiece Object Reference") (LevelGate :type "/Game/Game/LevelTransition/BP_LevelGate Object Reference"))
  (locals (CowPiece :type "/Game/LevelCreation/BP_CowHUBPiece Object Reference") (ObtainedCow :type Boolean) (CowData :type "/Game/LevelCreation/Pickups/STRUCT_CowCollectible Structure") (Gate :type "/Game/Game/LevelTransition/BP_LevelGate Object Reference"))
  (bind _returnvalue (`KismetStringLibrary.Conv_StringToName` (`KismetSystemLibrary.GetDisplayName` (`local.CowPiece`))))
  (set `local.CowPiece` Cow)
  (set `local.ObtainedCow` Obtained)
  (set `local.Gate` LevelGate)
  (`|ExecutionSequence`
    (:`then_0`
      ;[1 1 1] Checking cow obtained from game instance
      (if (not (`self.OverrideCowData`))
        (bind _collectibleobtained_ (`/Game/Game/BP_GameInstance.HasCowBeenObtained` (`self.GameInstance`) _returnvalue))
        (bind _output_get (set `local.ObtainedCow` _collectibleobtained_))
        (if _output_get
          (bind _cow_data (`/Game/Game/BP_GameInstance.GetCowData` (`self.GameInstance`) _returnvalue))
          (set `local.CowData` _cow_data))))
    (:`then_1`
      ;[1 1 1] Locking/unlocking cow based on game instance data
      (if (`local.ObtainedCow`)
        (`/Game/LevelCreation/BP_CowHUBPiece.Unlock` (`local.CowPiece`))
        (`/Game/Game/LevelTransition/BP_LevelGate.SetCowLabelState` (`local.LevelGate`))
        (if (not (`self.OverrideCowData`))
          (`/Game/LevelCreation/BP_CowHUBPiece.SetupAnimations` (`local.CowPiece`) (`local.CowData`)))
        (else
          (`/Game/LevelCreation/BP_CowHUBPiece.Lock` (`local.CowPiece`)))))))

(fn `SetupLevel`
  (params (LevelParams :type "/Game/Game/LevelTransition/STRUCT_LevelTransitionParameters Structure"))
  (locals (Level :type "/Game/Game/LevelTransition/STRUCT_LevelTransitionParameters Structure") (HUBPiece :type "/Game/LevelCreation/HUB/BP_HUBPiece Object Reference") (LevelGate :type "/Game/Game/LevelTransition/BP_LevelGate Object Reference"))
  ;[1 1 1] Setup local parameters
  (bind _output_get (set `local.Level` LevelParams))
  (bind ((`HUBPiece_36_6CCF174C49F03093BAE381AB7D9BD947` _hubpiece) (`LevelGate_33_37F0881240130F38A98BDEBF03AA7C9F` _levelgate)) (break `/Game/Game/LevelTransition/STRUCT_LevelTransitionParameters` _output_get))
  (set `local.HUBPiece` _hubpiece)
  (set `local.LevelGate` _levelgate)
  (`|ExecutionSequence`
    (:`then_0`
      ;[1 1 1] Get level completion state and optional collectibles from game instance
      (bind _level_state (`/Game/Game/BP_GameInstance.GetLevelState` (`self.GameInstance`) (`.LevelName_24_50A6B0C84C53A264E6DBD4BF8EF57C39` (break `/Game/Game/LevelTransition/STRUCT_LevelTransitionParameters` (`local.Level`)))))
      (setmembers `/Game/Game/LevelTransition/STRUCT_LevelTransitionParameters` :`StructRef` (`local.Level`) :`Level State` _level_state)
      (if (`self.OverrideLevelData`)
        (if (`|EnumInequality` (`.LevelState_35_92F39F3E426DB084083709958D29A340` (break `/Game/Game/LevelTransition/STRUCT_LevelTransitionParameters` (`local.Level`))) "NewEnumerator2")
          (setmembers `/Game/Game/LevelTransition/STRUCT_LevelTransitionParameters` :`StructRef` (`local.Level`) :`Level State` "NewEnumerator1"))))
    (:`then_1`
      ;[1 1 1] Check Level unlocked
      (switch `/Game/Game/LevelTransition/ENUM_LevelState` (`.LevelState_35_92F39F3E426DB084083709958D29A340` (break `/Game/Game/LevelTransition/STRUCT_LevelTransitionParameters` (`local.Level`)))
        (:`NewEnumerator0`
          (`self.LockLevel` (`local.Level`))
          (`/Game/LevelCreation/HUB/BP_HUBPiece.Lock` (`local.HUBPiece`)))
        (:`NewEnumerator1`
          (`self.UnlockLevel` (`local.Level`))
          (`/Game/LevelCreation/HUB/BP_HUBPiece.Lock` (`local.HUBPiece`))
          (`/Game/Game/LevelTransition/BP_LevelGate.SetFurnitureLabelState` (`local.LevelGate`) "NewEnumerator1"))
        (:`NewEnumerator2`
          (`self.UnlockLevel` (`local.Level`))
          (`/Game/LevelCreation/HUB/BP_HUBPiece.Unlock` (`local.HUBPiece`))
          (`/Game/Game/LevelTransition/BP_LevelGate.SetFurnitureLabelState` (`local.LevelGate`) "NewEnumerator2"))))))

(fn `SetupLevels`
  (locals (LevelSettings :type "/Game/Game/LevelTransition/STRUCT_LevelTransitionParameters Structure") (LevelIndex :type Integer))
  (bind ((`CowObtained_39_E62998D744B41B4C0D7C95AB5577953D` _cowobtained) (`CowHUBPiece_44_695426B94908C51143DD818F43E1613F` _cowhubpiece) (`LevelGate_33_37F0881240130F38A98BDEBF03AA7C9F` _levelgate)) (break `/Game/Game/LevelTransition/STRUCT_LevelTransitionParameters` (`local.LevelSettings`)))
  (`|ExecutionSequence`
    (:`then_0`
      ;[1 1 1] Unlock levels for showcase
      (set `self.OverrideLevelData` (`/Game/Game/BP_GameInstance.AllLevelsUnlocked` (`self.GameInstance`))))
    (:`then_1`
      (for (_array_element _array_index) (`self.Levels`)
        (set `local.LevelIndex` _array_index)
        (bind _output_get (set `local.LevelSettings` _array_element))
        (`self.SetupLevel` _output_get)
        (`self.SetupCow` _cowobtained _cowhubpiece _levelgate)
        ;[1 1 1] Add reference to transition index for identification
        (`BlueprintMapLibrary.Map_Add` (`self.Transitions`) (`.LevelTransitionPlatform_25_F3C83AF7499F67344C459C905D6240B8` (break `/Game/Game/LevelTransition/STRUCT_LevelTransitionParameters` (`local.LevelSettings`))) (`local.LevelIndex`))))))

(fn `SetupPlatformDefaults`
  (params (TransitionPlatform :type "/Game/Platforms/BP_Killable Object Reference"))
  (set `/Game/Platforms/BP_Killable.Incapacitate` true TransitionPlatform)
  (set `/Game/Platforms/BP_Platform.ActivationBehavior` "NewEnumerator2" TransitionPlatform))

(fn `UnlockLevel`
  (params (Level :type "/Game/Game/LevelTransition/STRUCT_LevelTransitionParameters Structure"))
  (bind ((`LevelTransitionPlatform_25_F3C83AF7499F67344C459C905D6240B8` _leveltransitionplatform) (`LevelGate_33_37F0881240130F38A98BDEBF03AA7C9F` _levelgate)) (break `/Game/Game/LevelTransition/STRUCT_LevelTransitionParameters` Level))
  (`/Game/Game/LevelTransition/BP_LevelGate.UnlockGate` _levelgate)
  (`self.AddLevelTransition` Level)
  (`self.SetupPlatformDefaults` _leveltransitionplatform))

(fn `UserConstructionScript`)