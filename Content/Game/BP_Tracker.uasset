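; BP_Tracker overrides the player's unlockables when play begins, based on its own double jump and sprint flags.
; It caches the game mode, game instance and player controller, then calls the game instance's unlock function for each enabled flag.
; If either flag sets the override, it has the player controller assign the unlockables to the player.
; The OverrideUnlocks function and construction script are empty.
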(event `self.ReceiveBeginPlay`
  (`self.SetupReferences`)
  (`self.SetupUnlockables`))

(fn `OverrideUnlocks`
  (locals (OverrideCurrentPlayer :type Boolean)))

(fn `SetupReferences`
  (bind _asbp_game_mode (cast `/Game/Game/BP_GameMode` (`GameplayStatics.GetGameMode`)))
  (set `self.GameMode` _asbp_game_mode)
  (bind _asbp_game_instance (cast `/Game/Game/BP_GameInstance` (`GameplayStatics.GetGameInstance`)))
  (set `self.GameInstance` _asbp_game_instance)
  (bind _asbp_player_controller (cast `/Game/Player/BP_PlayerController` (`GameplayStatics.GetPlayerController` 0)))
  (set `self.PlayerController` _asbp_player_controller))

(fn `SetupUnlockables`
  (locals (Override :type Boolean))
  ;[1 1 1] Check to see if player's unlockables is to be overridden
  (`|ExecutionSequence`
    (:`then_0`
      (if (`self.UnlockDoubleJump`)
        (set `local.Override` true)
        (`/Game/Game/BP_GameInstance.UnlockDoubleJump` (`self.GameInstance`))))
    (:`then_1`
      (if (`self.UnlockSprint`)
        (set `local.Override` true)
        (`/Game/Game/BP_GameInstance.UnlockSprint` (`self.GameInstance`))))
    (:`then_2`
      (if (`local.Override`)
        (`/Game/Player/BP_PlayerController.AssignUnlockablesToPlayer` (`self.PlayerController`) true)))))

(fn `UserConstructionScript`)