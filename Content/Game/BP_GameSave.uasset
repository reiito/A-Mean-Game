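; BP_GameSave is a data container for the player's saved progress and settings, covering ability unlocks, invert and mute options, completion and cheat flags, death count, level states, cow collectibles and play time.
; SetAllVariables writes every field at once from its inputs, using a Sequence node to group related assignments.
; ReturnAllVariables hands back the full set in one call, so the pair acts as a bulk setter and getter.
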(fn `ReturnAllVariables`
  (returns (DoubleJumpUnlocked :type Boolean) (SprintUnlocked :type Boolean) (Inverted :type Boolean) (Muted :type Boolean) (CheatsUsed :type Boolean) (GameCompleted :type Boolean) (EndShown :type Boolean) (OneLifeModeUnlocked :type Boolean) (DeathCount :type Integer) (CompletedLevelCount :type Integer) (LevelState :type "Map of Name to /Game/Game/LevelTransition/ENUM_LevelState Enum") (CowCollectibles :type "Map of Name to /Game/LevelCreation/Pickups/STRUCT_CowCollectible Structure") (TotalPlayTime :type "Float (double-precision)"))
  (return (`self.DoubleJumpUnlocked`) (`self.SprintUnlocked`) (`self.Inverted`) (`self.Muted`) (`self.CheatsUsed`) (`self.GameCompleted`) (`self.EndShown`) (`self.OneLifeModeUnlocked`) (`self.DeathCount`) (`self.CompletedLevelCount`) (`self.LevelState`) (`self.CowCollectibles`) (`self.TotalPlayTime`)))

(fn `SetAllVariables`
  (params (DoubleJumpUnlocked :type Boolean) (SprintUnlocked :type Boolean) (Inverted :type Boolean) (Muted :type Boolean) (CheatsUsed :type Boolean) (GameCompleted :type Boolean) (EndShown :type Boolean) (OneLifeModeUnlocked :type Boolean) (DeathCount :type Integer) (CompletedLevelCount :type Integer) (LevelState :type "Map of Name to /Game/Game/LevelTransition/ENUM_LevelState Enum") (CowCollectibles :type "Map of Name to /Game/LevelCreation/Pickups/STRUCT_CowCollectible Structure") (TotalPlayTime :type "Float (double-precision)"))
  (`|ExecutionSequence`
    (:`then_0`
      (set `self.DoubleJumpUnlocked` DoubleJumpUnlocked)
      (set `self.SprintUnlocked` SprintUnlocked))
    (:`then_1`
      (set `self.Inverted` Inverted)
      (set `self.Muted` Muted))
    (:`then_2`
      (set `self.CheatsUsed` CheatsUsed)
      (set `self.GameCompleted` GameCompleted)
      (set `self.EndShown` EndShown))
    (:`then_3`
      (set `self.DeathCount` DeathCount)
      (set `self.CompletedLevelCount` CompletedLevelCount))
    (:`then_4`
      (set `self.LevelState` LevelState)
      (set `self.CowCollectibles` CowCollectibles))
    (:`then_5`
      (set `self.TotalPlayTime` TotalPlayTime))
    (:`then_6`
      (set `self.OneLifeModeUnlocked` OneLifeModeUnlocked))))