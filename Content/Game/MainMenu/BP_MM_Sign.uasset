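; Main menu sign actor that opens on BeginPlay to reveal a widget screen for resume, new game, one-life mode, controls and quit.
; A timeline slides the top and bottom pieces apart and scales the screen, then enables input; Quit plays it in reverse before exiting.
; Throttled axis input navigates the widget, selection resets GameInstance as needed and loads the hub level.
; In editor, Delete clears the save.
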(event `self.ReceiveBeginPlay`
  ;[1 1 1] Setup sign
  (`/Game/Game/BP_Macros.SetupLerpTimeline` (`self.SignAnimation`) "/Game/Data/CURVEs/CURVE_LinearLerp.CURVE_LinearLerp" 1.0
    (:`__`
      (`self.Initialize`)
      (`self.OpenSign`))))

(event `OpenSign`
  ;[1 1 1] Play animation
  (bind _direction (`Timeline|SignAnimation` :!label _label)
    (:`Update`
      (`/Game/Game/BP_Macros.MoveComponent` (`self.SignTop`) (`KismetMathLibrary.MakeVector` 0.0 0.0 (+ (`self.HalfwayPoint`) (`self.Offset`))) (`KismetMathLibrary.MakeVector` 0.0 0.0 (`self.DistanceApart`)) (`self.SignAnimation`) true
        (:`__`
          (`/Game/Game/BP_Macros.MoveComponent` (`self.SignBottom`) (`KismetMathLibrary.MakeVector` 0.0 0.0 (- (`self.HalfwayPoint`) (`self.Offset`))) (0.0 0.0 0.0) (`self.SignAnimation`) true
            (:`__`
              (`SceneComponent.SetRelativeScale3D` (`self.Screen`) (`KismetMathLibrary.VLerp` (`self.ClosedScreenSize`) (`self.OpenedScreenSize`) (`TimelineComponent.GetPlaybackPosition` (`self.SignAnimation`)))))))))
    (:`Finished`
      (if (`|EnumEquality` _direction "Forward")
        (`/Game/Game/MainMenu/Data/BP_MM_SignUI.ShowScreen` (`self.ScreenUI`))
        (set `self.InputEnabled` true)
        (else
          (`KismetSystemLibrary.QuitGame` null "Quit"))))))

(event `CloseSignAndQuit`
  ;[1 1 1] Play animation
  (`/Game/Game/MainMenu/Data/BP_MM_SignUI.HideScreen` (`self.ScreenUI`))
  (set `self.InputEnabled` false)
  (goto _label :!via `ReverseFromEnd`))

(event `InputAction|SelectMenuItem`
  (params (Key :type "Key Structure"))
  ;[1 1 1] Input
  (:`Pressed`
    (if (`self.InputEnabled`)
      (set `self.IsController` (`KismetInputLibrary.Key_IsGamepadKey` Key))
      (switch `/Game/Game/MainMenu/Data/ENUM_MM_Selected` (`/Game/Game/MainMenu/Data/BP_MM_SignUI.CurrentOption` (`self.ScreenUI`))
        (:`NewEnumerator6`
          (`self.ResumeGame`))
        (:`NewEnumerator0`
          (`self.NewGame`))
        (:`NewEnumerator2`
          (`self.OpenOneLife Mode`))
        (:`NewEnumerator3`
          (`/Game/Game/MainMenu/Data/BP_MM_SignUI.ToggleControls` (`self.ScreenUI`) (`self.IsController`)))
        (:`NewEnumerator4`
          (`self.CloseSignAndQuit`))))))

(event `InputAxis|MainMenuInput`
  (params (AxisValue :type "Float (single-precision)"))
  ;[1 1 1] Input
  (if (and (!= AxisValue 0.0) (`self.InputEnabled`) (not (`/Game/Game/MainMenu/Data/BP_MM_SignUI.ViewingControls` (`self.ScreenUI`))))
    (`self.HandleMenuInput` AxisValue)))

(event `Key|Delete`
  (params (Key :type "Key Structure"))
  (:`Pressed`
    (if (`PlayerBPFL.InEditor`)
      (bind _asbp_game_instance (cast `/Game/Game/BP_GameInstance` (`GameplayStatics.GetGameInstance`)))
      (`/Game/Game/BP_GameInstance.ClearSave` _asbp_game_instance))))

(fn `Initialize`
  (bind _asbp_mm_sign_ui (cast `/Game/Game/MainMenu/Data/BP_MM_SignUI` (`WidgetComponent.GetUserWidgetObject` (`self.Screen`))))
  (set `self.ScreenUI` _asbp_mm_sign_ui)
  (`self.SetAnimationStartPosition`)
  (`/Game/Game/MainMenu/Data/BP_MM_SignUI.HideScreen` (`self.ScreenUI`))
  (bind _asbp_game_instance (cast `/Game/Game/BP_GameInstance` (`GameplayStatics.GetGameInstance`)))
  (set `self.GameInstanceReference` _asbp_game_instance))

(fn `NewGame`
  (bind _gameinstancereference (`self.GameInstanceReference`))
  (`/Game/Game/BP_GameInstance.ResetInstance` _gameinstancereference)
  (set `/Game/Game/BP_GameInstance.OneLifeMode` false _gameinstancereference)
  (`GameplayStatics.OpenLevel` "LVL_HUB"))

(fn `OpenOneLife Mode`
  (bind _gameinstancereference (`self.GameInstanceReference`))
  (`/Game/Game/BP_GameInstance.ResetInstance` _gameinstancereference)
  (set `/Game/Game/BP_GameInstance.OneLifeMode` true _gameinstancereference)
  (`GameplayStatics.OpenLevel` "LVL_HUB"))

(fn `ResumeGame`
  (`GameplayStatics.OpenLevel` "LVL_HUB"))

(fn `SetAnimationStartPosition`
  (locals (HalfwayPoint2 :type "Float (double-precision)"))
  ;[1 1 1] Set base positions for sign top and bottom
  (`SceneComponent.SetRelativeScale3D` (`self.Screen`) (`self.ClosedScreenSize`))
  (`SceneComponent.K2_SetRelativeLocation` (`self.SignTop`) (`KismetMathLibrary.MakeVector` 0.0 0.0 (+ (`self.HalfwayPoint`) (`self.Offset`))) false false)
  (`SceneComponent.K2_SetRelativeLocation` (`self.SignBottom`) (`KismetMathLibrary.MakeVector` 0.0 0.0 (- (`self.HalfwayPoint`) (`self.Offset`))) false false))

(fn `UserConstructionScript`
  (`SceneComponent.SetRelativeScale3D` (`self.Screen`) (`self.OpenedScreenSize`))
  (`SceneComponent.SetRelativeScale3D` (`self.Layout`) (`self.Size`))
  (set `self.HalfwayPoint` (/ (`self.DistanceApart`) 2.0))
  (`SceneComponent.K2_SetRelativeLocation` (`self.ScreenLayout`) (`KismetMathLibrary.MakeVector` 0.0 0.0 (+ (`self.HalfwayPoint`) (* (`self.Offset`) 2.5))) false false))