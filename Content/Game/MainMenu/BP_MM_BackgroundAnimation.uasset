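; Main menu background actor that loops a scene of a dead body being swapped for a character on a moving platform.
; An AnimationStage state machine chains lerp timelines: the platform slides and rotates, and a spinning Switcher moves in and later reverses out.
; SwitchBodies replaces the spawned dead body with a character attached to the platform.
; The platform then moves across and up, destroys the character and restarts the cycle.
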(event `SwitchState`
  ;[1 1 1] Swapping between animation states
  (switch `/Game/Game/MainMenu/Data/ENUM_MM_AnimationState` (`self.AnimationStage`)
    (:`NewEnumerator3`
      ;[1 1 1] Spawn dead character then move across
      (bind _returnvalue (`|SpawnActorFromClass` "/Game/Game/MainMenu/Meshes/BP_MM_DeadCharacter.BP_MM_DeadCharacter_C" (`KismetMathLibrary.MakeTransform` (`SceneComponent.K2_GetComponentLocation` (`self.Right-DeadBodySpawnPoint`)) (struct :`Roll` 180.0)) "Undefined" "OverrideRootScale" null null))
      (set `self.SpawnedBody` _returnvalue)
      (`KismetSystemLibrary.Delay` 4.0)
      (set `self.AnimationStage` "NewEnumerator0")
      (`self.MovePlatform`))
    (:`NewEnumerator0`
      (set `self.AnimationStage` "NewEnumerator1")
      (`self.PlayStage2`))
    (:`NewEnumerator1`
      (set `self.AnimationStage` "NewEnumerator2")
      (`self.PlayStage3`))))

(event `MovePlatform`
  ;[1 1 1] Reused, move platform across
  (`Timeline|Move Platform Across` :!via `PlayFromStart`
    (:`Update`
      (`/Game/Game/BP_Macros.MoveComponent` (`self.Platform`) (`self.PlatformCurrPos`) (+ (`self.PlatformCurrPos`) (`self.MoveAcrossDistance`)) (`self.Move Platform Across`) true
        (:`__`
          (`self.RotatePlatform`))))
    (:`Finished`
      (set `self.PlatformCurrPos` (+ (`self.PlatformCurrPos`) (`self.MoveAcrossDistance`)))
      (`KismetSystemLibrary.Delay` 1.0)
      (`self.SwitchState`))))

(event `self.ReceiveBeginPlay`
  (`/Game/Game/BP_Macros.SetupLerpTimeline` (`self.Move Platform Across`) "/Game/Data/CURVEs/CURVE_LinearLerp.CURVE_LinearLerp" 0.75
    (:`__`
      (`/Game/Game/BP_Macros.SetupLerpTimeline` (`self.Switch to new body`) "/Game/Data/CURVEs/CURVE_LinearLerp.CURVE_LinearLerp" 0.75
        (:`__`
          (`/Game/Game/BP_Macros.SetupLerpTimeline` (`self.Move Platform Up`) "/Game/Data/CURVEs/CURVE_LinearLerp.CURVE_LinearLerp" 0.75
            (:`__`
              (`self.PlayBackgroundAnimation`))))))))

(event `PlayBackgroundAnimation`
  (set `self.AnimationStage` "NewEnumerator3")
  (set `self.PlatformCurrPos` (`self.PlatformStartPos`))
  (`self.MovePlatform`))

(event `PlayStage2`
  ;[1 1 1] Stage 2 behaviour: Move switcher down, spiralling motion
  (bind _direction (`Timeline|Switch to new body` :!via `PlayFromStart` :!label _label)
    (:`Update`
      (`SceneComponent.K2_SetRelativeRotation` (`self.Switcher`) (`KismetMathLibrary.RLerp` (struct :`Yaw` -180.0) (struct) (`TimelineComponent.GetPlaybackPosition` (`self.Switch to new body`))) false false)
      (`/Game/Game/BP_Macros.MoveComponent` (`self.Switcher`) (0.0 0.0 0.0) (`self.SwitcherMoveDistance`) (`self.Switch to new body`) true))
    (:`Finished`
      (if (`|EnumEquality` _direction "Forward")
        (`self.SwitchBodies`)
        (`KismetSystemLibrary.Delay` 2.0)
        (`self.ReverseSwitcher`)
        (`KismetSystemLibrary.Delay` 2.0)
        (`self.MovePlatform`)))))

(event `ReverseSwitcher`
  ;[1 1 1] Stage 2 behaviour: Move switcher down, spiralling motion
  (goto _label :!via `ReverseFromEnd`))

(event `PlayStage3`
  (bind _platformcurrpos (`self.PlatformCurrPos`))
  ;[1 1 1] Move platform + character up. Destroy when done and loop again from start
  (`Timeline|Move Platform Up` :!via `PlayFromStart`
    (:`Update`
      (`/Game/Game/BP_Macros.MoveComponent` (`self.Platform`) _platformcurrpos (+ _platformcurrpos (`self.MoveUpDistance`)) (`self.Move Platform Up`) true))
    (:`Finished`
      (`self.K2_DestroyActor` (`self.SpawnedCharacter`))
      (`self.PlayBackgroundAnimation`))))

(fn `RotatePlatform`
  (bind _platform (`self.Platform`))
  (bind _returnvalue (`TimelineComponent.GetPlaybackPosition` (`self.Move Platform Across`)))
  (switch `/Game/Game/MainMenu/Data/ENUM_MM_AnimationState` (`self.AnimationStage`)
    (:`NewEnumerator0`
      (`SceneComponent.K2_SetRelativeRotation` _platform (`KismetMathLibrary.RLerp` (struct :`Yaw` 90.0) (struct :`Yaw` 60.0) _returnvalue) false false))
    (:`NewEnumerator1`
      (`SceneComponent.K2_SetRelativeRotation` _platform (`KismetMathLibrary.RLerp` (struct :`Yaw` 60.0) (struct :`Yaw` 90.0) _returnvalue) false false))))

(fn `SetupVariables`
  (set `self.PlatformStartPos` (`SceneComponent.RelativeLocation` (`self.Platform`))))

(fn `SwitchBodies`
  (`self.K2_DestroyActor` (`self.SpawnedBody`))
  (bind _returnvalue (`|SpawnActorFromClass` "/Game/Game/MainMenu/Meshes/BP_MM_Character.BP_MM_Character_C" (`KismetMathLibrary.MakeTransform` (+ (`SceneComponent.K2_GetComponentLocation` (`self.Platform`)) (0.0 0.0 10.0)) (struct :`Yaw` 180.0)) "Undefined" "OverrideRootScale" null null))
  (bind _output_get (set `self.SpawnedCharacter` _returnvalue))
  (`self.K2_AttachToComponent` _output_get (`self.Platform`) "None" "KeepWorld" "KeepWorld" "KeepWorld" true))

(fn `UserConstructionScript`
  (`self.SetupVariables`))