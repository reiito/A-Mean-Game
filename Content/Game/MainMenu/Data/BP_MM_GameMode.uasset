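; Main menu GameMode that triggers save loading through BP_GameInstance on BeginPlay.
; On the first run it sets the instance's Loaded flag, initializes the save game object and loads the full game.
; On later runs it reloads only if OneLifeMode is set, clearing that flag first.
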(event `self.ReceiveBeginPlay`
  (bind _gameinstanceref (`self.GameInstanceRef`))
  (bind _asbp_game_instance (cast `/Game/Game/BP_GameInstance` (`GameplayStatics.GetGameInstance`)))
  (bind _output_get (set `self.GameInstanceRef` _asbp_game_instance))
  (if (`/Game/Game/BP_GameInstance.Loaded` _output_get)
    (if (`/Game/Game/BP_GameInstance.OneLifeMode` _gameinstanceref)
      (set `/Game/Game/BP_GameInstance.OneLifeMode` false _gameinstanceref)
      (`/Game/Game/BP_GameInstance.LoadFullGame` _output_get :!label _label))
    (else
      (set `/Game/Game/BP_GameInstance.Loaded` true _output_get)
      (`/Game/Game/BP_GameInstance.InitSaveGameObject` _output_get)
      (goto _label))))

(fn `UserConstructionScript`)