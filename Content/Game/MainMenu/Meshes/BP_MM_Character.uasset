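; Main menu character Blueprint that drives a blend value for randomly chosen gestures.
; BeginPlay configures the GestureBlender timeline with a linear lerp curve and blend speed.
; PlayGesture picks a random index within twice the gesture count, bumps odd results to even, then restarts the timeline.
; Timeline updates use playback position to lerp AnimBlendValue from that index to the next.
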(event `self.ReceiveBeginPlay`
  (`/Game/Game/BP_Macros.SetupLerpTimeline` (`self.GestureBlender`) "/Game/Data/CURVEs/CURVE_LinearLerp.CURVE_LinearLerp" (`self.BlendSpeed`)))

(fn `PlayGesture`
  (bind _returnvalue (* (`self.GestureCount`) 2))
  (`|ExecutionSequence`
    (:`then_0`
      (bind _output_get (set `self.BlendIndex` (`KismetMathLibrary.RandomIntegerInRange` 0 _returnvalue)))
      (if (> (mod _output_get 2) 0)
        (if (== _output_get _returnvalue)
          (set `self.BlendIndex` (- _output_get 1))
          (else
            (set `self.BlendIndex` (+ _output_get 1))))))
    (:`then_1`
      (`TimelineComponent.PlayFromStart` (`self.GestureBlender`)))))

(fn `UserConstructionScript`)