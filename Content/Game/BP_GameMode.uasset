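; Game mode that manages a level run: run timer, total play time, death and restart counts, respawning and level transitions.
; It caches the player controller, game instance and HUD widget, forwarding level name, unlock, cheat, game-over and main-menu displays to the HUD.
; Level transitions chain a looping UpdateText macro that types thirteen loading-screen lines character by character, randomly scrambling characters, then open the requested level.
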(event `self.ReceiveBeginPlay`
  ;[1 1 1] Startup
  (`self.SetupReferences`)
  (`self.StartRunTimer`)
  (`self.ViewLevelName`))

(event `StartRunTimer`
  ;[1 1 1] Timer - Log how long player took
  (bind (_direction _timetaken) (`Timeline|RunTimeline` :!label _label)
    (:`Update`
      (set `self.TimeTaken` _timetaken))))

(event `RunLevelTransition`
  (params (RandomCharacterChance :type "Float (double-precision)") (`Level Name` :type Name))
  ;[1 1 1] Load all lines in loading screen
  (set `self.ChanceForRandomCharacter` RandomCharacterChance)
  (`/Game/Game/BP_UI.ViewLoadingScreen` (`self.HUDWidget`))
  (`self.UpdateText` (`|GetArrayItem` (`self.LoadingScreenLines`)) (`self.LoadingLine1`)
    (:`Done`
      (`self.UpdateText` (`|GetArrayItem` (`self.LoadingScreenLines`) 1) (`self.LoadingLine2`)
        (:`Done`
          (`self.UpdateText` (`|GetArrayItem` (`self.LoadingScreenLines`) 2) (`self.LoadingLine3`)
            (:`Done`
              (`self.UpdateText` (`|GetArrayItem` (`self.LoadingScreenLines`) 3) (`self.LoadingLine4`)
                (:`Done`
                  (`self.UpdateText` (`|GetArrayItem` (`self.LoadingScreenLines`) 4) (`self.LoadingLine5`)
                    (:`Done`
                      (`self.UpdateText` (`|GetArrayItem` (`self.LoadingScreenLines`) 5) (`self.LoadingLine6`)
                        (:`Done`
                          (`self.UpdateText` (`|GetArrayItem` (`self.LoadingScreenLines`) 6) (`self.LoadingLine7`)
                            (:`Done`
                              (`self.UpdateText` (`|GetArrayItem` (`self.LoadingScreenLines`) 7) (`self.LoadingLine8`)
                                (:`Done`
                                  (`self.UpdateText` (`|GetArrayItem` (`self.LoadingScreenLines`) 8) (`self.LoadingLine9`)
                                    (:`Done`
                                      (`self.UpdateText` (`|GetArrayItem` (`self.LoadingScreenLines`) 9) (`self.LoadingLine10`)
                                        (:`Done`
                                          (`self.UpdateText` (`|GetArrayItem` (`self.LoadingScreenLines`) 10) (`self.LoadingLine11`)
                                            (:`Done`
                                              (`self.UpdateText` (`|GetArrayItem` (`self.LoadingScreenLines`) 11) (`self.LoadingLine12`)
                                                (:`Done`
                                                  (`self.UpdateText` (`|GetArrayItem` (`self.LoadingScreenLines`) 12) (`self.LoadingLine13`)
                                                    (:`Done`
                                                      (`GameplayStatics.OpenLevel` `Level Name`))))))))))))))))))))))))))))

(event `StopRunTimer`
  ;[1 1 1] Timer - Log how long player took
  (goto _label :!via `Stop`))

(event `self.ReceiveTick`
  (params (DeltaSeconds :type "Float (single-precision)"))
  (bind _player (`self.Player`))
  (`/Engine/EditorBlueprintResources/StandardMacros.IsValid` _player
    (:`Is Valid`
      (if (`|EnumEquality` (`/Game/Player/BP_Character.InputDirectedTo` _player) "NewEnumerator2")
        (`/Game/Game/BP_GameInstance.AddToTotalTimePlayed` (`self.GameInstance`))))
    (:`Is Not Valid`
      (set `self.Player` (`/Game/Player/BP_PlayerController.CurrentCharacter` (`self.PlayerController`))))))

(fn `ActivatedCheat`
  (params (CheatMessage :type String))
  (`/Game/Game/BP_UI.ViewCheatPopup` (`self.HUDWidget`) CheatMessage))

(fn `ChangeControlDisplay`
  (params (Controller :type Boolean))
  ;[1 1 1] Xbox controller
  (if Controller
    (set `self.KeyboardVis` "Hidden")
    (set `self.XBoxVis` "Visible")
    (else
      (set `self.XBoxVis` "Hidden")
      (set `self.KeyboardVis` "Visible"))))

(fn `CowObtained`
  (params (CowImage :type "Texture2D Object Reference") (Message :type String))
  (`/Game/Game/BP_UI.ViewCowObtainedPopup` (`self.HUDWidget`) CowImage Message))

(fn `DiedInOneLifeMode`
  (`/Game/Game/BP_UI.ViewGameOverPopup` (`self.HUDWidget`)))

(fn `DoubleJumpObtained`
  (`/Game/Game/BP_UI.ViewDoubleJumpPopup` (`self.HUDWidget`)))

(fn `IncrementSavedData`
  (params (Type :type "/Game/Data/ENUMs/ENUM_SavedDataType Enum" :default "NewEnumerator0"))
  (switch `/Game/Data/ENUMs/ENUM_SavedDataType` Type
    (:`NewEnumerator0`
      (`/Engine/EditorBlueprintResources/StandardMacros.IncrementInt` (`self.NumDeaths`)))
    (:`NewEnumerator1`
      (`/Engine/EditorBlueprintResources/StandardMacros.IncrementInt` (`self.NumRestarts`)))))

(fn `Respawn`
  (`self.ResetLevel`)
  (`/Game/Player/BP_PlayerController.SpawnCharacter` (`self.PlayerController`)))

(fn `ReturnToMainMenu`
  (`/Game/Game/BP_UI.ViewTransitionToMainMenu` (`self.HUDWidget`)))

(fn `SaveRun`
  (`self.StopRunTimer`)
  (`GameplayStatics.GetCurrentLevelName` true))

(fn `SetupReferences`
  (bind _widget_reference (`/Game/Game/BP_Macros.AddHudWidget` "/Game/Game/BP_UI.BP_UI_C")
    (:`__`
      (bind _asbp_ui (cast `/Game/Game/BP_UI` _widget_reference))
      (set `self.HUDWidget` _asbp_ui)
      (bind _asbp_player_controller (cast `/Game/Player/BP_PlayerController` (`GameplayStatics.GetPlayerController` 0)))
      (bind _output_get (set `self.PlayerController` _asbp_player_controller))
      (set `self.Player` (`/Game/Player/BP_PlayerController.CurrentCharacter` _output_get))
      (bind _asbp_game_instance (cast `/Game/Game/BP_GameInstance` (`GameplayStatics.GetGameInstance`)))
      (set `self.GameInstance` _asbp_game_instance))))

(fn `SprintObtained`
  (`/Game/Game/BP_UI.ViewSprintPopup` (`self.HUDWidget`)))

(fn `UserConstructionScript`)

(fn `ViewLevelName`
  (bind _returnvalue (`GameplayStatics.GetCurrentLevelName` true))
  (bind (_value _returnvalue_2) (`BlueprintMapLibrary.Map_Find` (`self.LevelNames`) _returnvalue))
  (if _returnvalue_2
    (set `self.LevelName` _value)
    (`/Game/Game/BP_UI.ViewLevelName` (`self.HUDWidget`))))