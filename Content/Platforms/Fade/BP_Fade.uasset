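; Platform Blueprint that fades out as its inherited animation plays and can optionally stop blocking Pawns once faded.
; Construction creates three dynamic fade material instances for the body, icon and corners.
; Animation updates lerp their Fade parameter from default opacity to zero by playback position, while finish and reverse events toggle Pawn collision.
; Enable and disable overrides switch only the step trigger's Pawn overlap response.
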(event `self.Animation__UpdateFunc`
  ;[1 1 1] Animation
  (`self.UpdateOpacity`))

(event `self.FinishReversing`
  ;[1 1 1] Toggle interaction
  (`parent.FinishReversing`)
  (if (`self.DisableCollisionOnFade`)
    (`PrimitiveComponent.SetCollisionResponseToChannel` (`self.Platform`) "ECC_Pawn" "ECR_Block")))

(event `self.FinishAnimation`
  ;[1 1 1] Toggle interaction
  (`parent.FinishAnimation`)
  (if (`self.DisableCollisionOnFade`)
    (`PrimitiveComponent.SetCollisionResponseToChannel` (`self.Platform`) "ECC_Pawn" "ECR_Ignore")))

(event `self.EnablePlatform`
  ;[1 1 1] Override icon setting/removal in enabling/disabling platform
  (`PrimitiveComponent.SetCollisionResponseToChannel` (`self.StepTrigger`) "ECC_Pawn" "ECR_Overlap"))

(event `self.DisablePlatform`
  ;[1 1 1] Override icon setting/removal in enabling/disabling platform
  (`PrimitiveComponent.SetCollisionResponseToChannel` (`self.StepTrigger`) "ECC_Pawn" "ECR_Ignore"))

(fn `FadeMaterialInstance`
  (params (`Material Instance` :type "MaterialInstanceDynamic Object Reference"))
  (`MaterialInstanceDynamic.SetScalarParameterValue` `Material Instance` "Fade" (`KismetMathLibrary.Lerp` (`self.DefaultOpacity`) 0.0 (`TimelineComponent.GetPlaybackPosition` (`self.Animation`)))))

(fn `SetupFadingTextures`
  ;[1 1 1] Setup textures to fade
  ;;[1 1 1] Platform's white section
  (bind _returnvalue (`PrimitiveComponent.CreateDynamicMaterialInstance` (`self.Platform`) 0 "/Game/Platforms/Fade/MAT_FadeEffect.MAT_FadeEffect"))
  (bind _output_get (set `self.MaterialInstance0` _returnvalue))
  (`MaterialInstanceDynamic.SetTextureParameterValue` _output_get "Texture" (`self.PlatformTexture`))
  ;;[1 1 1] Icon itself
  (bind _returnvalue_2 (`PrimitiveComponent.CreateDynamicMaterialInstance` (`self.Platform`) 1 "/Game/Platforms/Fade/MAT_FadeEffect.MAT_FadeEffect"))
  (bind _output_get_2 (set `self.MaterialInstance1` _returnvalue_2))
  (`MaterialInstanceDynamic.SetTextureParameterValue` _output_get_2 "Texture" (`self.IconSprite`))
  ;;[1 1 1] Corners
  (bind _returnvalue_3 (`PrimitiveComponent.CreateDynamicMaterialInstance` (`self.Platform`) 2 "/Game/Platforms/Fade/MAT_FadeEffect.MAT_FadeEffect"))
  (bind _output_get_3 (set `self.MaterialInstance2` _returnvalue_3))
  (`MaterialInstanceDynamic.SetTextureParameterValue` _output_get_3 "Texture" (`self.CornerTexture`)))

(fn `UpdateOpacity`
  (bind _returnvalue (`KismetMathLibrary.Lerp` (`self.DefaultOpacity`) 0.0 (`TimelineComponent.GetPlaybackPosition` (`self.Animation`))))
  (`MaterialInstanceDynamic.SetScalarParameterValue` (`self.MaterialInstance0`) "Fade" _returnvalue)
  (`MaterialInstanceDynamic.SetScalarParameterValue` (`self.MaterialInstance1`) "Fade" _returnvalue)
  (`MaterialInstanceDynamic.SetScalarParameterValue` (`self.MaterialInstance2`) "Fade" _returnvalue))

(fn `UserConstructionScript`
  (`parent.UserConstructionScript`)
  (`self.SetupFadingTextures`))