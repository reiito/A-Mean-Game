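; Base step-triggered platform that plays a lerp timeline, with empty update and finish functions as hooks for child platforms to override.
; Player overlap or activate-on-play starts it, and the activation setting makes it retrigger, loop or fire once, optionally reversing.
; A reset setting binds reverse, jump-to-start, stop, re-enable or disable handlers to reset and completion events.
; Construction applies mesh, icon, orientation, visibility and trigger bounds.
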(event `SetResetBehaviour`
  ;[1 1 1] Resetting
  (switch `/Game/Platforms/ENUM_ResetBehaviour` (`self.ResetBehaviour`)
    (:`NewEnumerator5`
      (`self.ReverseAnimationOnReset`)
      (`self.ReEnableTriggerOnReset` :!label _label))
    (:`NewEnumerator6`
      (`self.JumpToInitialStateOnReset`)
      (goto _label))
    (:`NewEnumerator0`
      (`self.ReverseAnimationOnReset`)
      (`self.DisableOnReset` :!label _label_2))
    (:`NewEnumerator1`
      (`self.JumpToInitialStateOnReset`)
      (goto _label_2))
    (:`NewEnumerator4`
      (`self.StopOnReset`))))

(event `ReverseAnimationOnReset`
  ;[1 1 1] Resetting
  ;;[1 1 1] Resetting events to bind
  (if (`|EnumInequality` (`self.ActivationBehavior`) "NewEnumerator3")
    (add `self.Reset` (delegate `ReverseOnReset`))))

(event `ReverseOnReset`
  ;[1 1 1] Resetting
  ;;[1 1 1] Resetting events to bind
  (`TimelineComponent.ReverseFromEnd` (`self.Animation`)))

(event `JumpToInitialStateOnReset`
  ;[1 1 1] Resetting
  ;;[1 1 1] Resetting events to bind
  (add `self.Reset` (delegate `JumpToInitialState`)))

(event `self.K2_OnReset`
  ;[1 1 1] Resetting
  (if (`self.Activated`)
    (`self.Reset`)
    (set `self.Activated` false)))

(event `JumpToInitialState`
  ;[1 1 1] Resetting
  ;;[1 1 1] Resetting events to bind
  (`TimelineComponent.SetNewTime` (`self.Animation`) 0.0))

(event `DisableOnReset`
  ;[1 1 1] Resetting
  ;;[1 1 1] Resetting events to bind
  (add `self.Reset` (delegate `ResetDisable`)))

(event `ResetDisable`
  ;[1 1 1] Resetting
  ;;[1 1 1] Resetting events to bind
  (`self.DisableOnResetBehaviour`))

(event `ReEnableTriggerOnReset`
  ;[1 1 1] Resetting
  ;;[1 1 1] Resetting events to bind
  (add `self.Reset` (delegate `ReEnableTrigger`)))

(event `StopOnReset`
  ;[1 1 1] Resetting
  (add `self.Reset` (delegate `StopAnimation`)))

(event `self.ReceiveBeginPlay`
  ;[1 1 1] Setup
  (`self.Initialize`)
  (`/Game/Game/BP_Macros.SetupLerpTimeline` (`self.Animation`) "/Game/Data/CURVEs/CURVE_LinearLerp.CURVE_LinearLerp" (`self.AnimationSpeed`)))

(event `ReEnableTrigger`
  ;[1 1 1] Resetting
  ;;[1 1 1] Resetting events to bind
  (`self.EnablePlatform`)
  (`self.ResetStepTriggerDisabling`))

(event `StopAnimation`
  ;[1 1 1] Resetting
  (`TimelineComponent.Stop` (`self.Animation`))
  (`self.DisableOnReset`))

(event `ReverseWhenDone`
  ;[1 1 1] Perform reverse when animation finishes
  (add `self.AnimationDone` (delegate `ReverseBehaviour`)))

(event `DisableStepTriggerWhenDone`
  ;[1 1 1] Add behaviour on end animation to also disable step trigger
  (add `self.AnimationDone` (delegate `DisableStepTriggerWhenDoneBehaviour`)))

(event `SetActivationBehaviour`
  ;[1 1 1] Activation Behaviour
  (`|ExecutionSequence`
    (:`then_0`
      (switch `/Game/Platforms/ENUM_ActivationBehaviour` (`self.ActivationBehavior`)
        (:`NewEnumerator2`
          (`self.EnablePlatform`)
          (`self.ReverseWhenDone`))
        (:`NewEnumerator3`
          (`self.CheckPlayerTriggerOnce`)
          (`self.Loop`))
        (:`NewEnumerator0`
          (`self.CheckPlayerTriggerOnce`))
        (:`NewEnumerator1`
          (`self.CheckPlayerTriggerOnce`)
          (`self.ReverseWhenDone`))))
    (:`then_1`
      (`self.IsActivatedOnPlay`
        (:`ActivatedOnPlay`
          (`self.Activate`))))))

(event `Loop`
  ;[1 1 1] Looping
  (add `self.ReverseDone` (delegate `ReactivateWhenReverseDone`))
  (`self.ReverseWhenDone`))

(event `DisableStepTriggerWhenDoneBehaviour`
  ;[1 1 1] Add behaviour on end animation to also disable step trigger
  (`/Engine/EditorBlueprintResources/StandardMacros.DoOnce` false :!label _label_3
    (:`Completed`
      (`self.DisablePlatform`))))

(event `ReverseBehaviour`
  ;[1 1 1] Perform reverse when animation finishes
  (`self.ReverseAnimation`))

(event `ReactivateWhenReverseDone`
  ;[1 1 1] Looping
  (`KismetSystemLibrary.Delay` (`self.LoopIterationDelay`))
  (`self.Activate`))

(event `ResetStepTriggerDisabling`
  ;[1 1 1] Add behaviour on end animation to also disable step trigger
  (goto _label_3 :!via `Reset`))

(event `self.StepTrigger.OnComponentBeginOverlap`
  (params (OverlappedComponent :type "PrimitiveComponent Object Reference") (OtherActor :type "Actor Object Reference") (OtherComp :type "PrimitiveComponent Object Reference") (OtherBodyIndex :type Integer) (bFromSweep :type Boolean) (SweepResult :type "HitResult Structure (by ref)"))
  ;[1 1 1] Activation
  (if (and (`/Game/Game/BP_Macros.IsPlayer` OtherActor) (not (`/Game/Game/BP_Macros.IsActiveTimeline` (`self.Animation`))))
    (`KismetSystemLibrary.Delay` (`self.StepOnActivationDelay`))
    (`self.Activate`)))

(fn `Activate`
  (set `self.Activated` true)
  (set `self.IsReversing` false)
  (`self.PlayNewTrggerSound` (`self.TrggerSound`))
  (`TimelineComponent.Play` (`self.Animation`)))

(fn `AnimationUpdate`)

(fn `CheckPlayerTriggerOnce`
  ;[1 1 1] Toggle Step Trigger depending on whether its activated on play
  (`self.IsActivatedOnPlay`
    (:`ActivatedOnPlay`
      (`self.DisablePlatform`))
    (:`RequireTrigger`
      (`self.EnablePlatform`)
      (`self.DisableStepTriggerWhenDone`))))

(fn `DeactivateIcon`
  (params (Component :type "StaticMeshComponent Object Reference"))
  (if (`|EnumInequality` (`self.ActivationBehavior`) "NewEnumerator3")
    (`PrimitiveComponent.SetMaterial` Component 1 (`self.BlankIconMaterial`))))

(fn `DisableOnResetBehaviour`
  (`self.DisablePlatform`))

(fn `DisablePlatform`
  (`PrimitiveComponent.SetCollisionResponseToChannel` (`self.StepTrigger`) "ECC_Pawn" "ECR_Ignore")
  (`self.DeactivateIcon` (`self.Platform`)))

(fn `EnablePlatform`
  (`PrimitiveComponent.SetCollisionResponseToChannel` (`self.StepTrigger`) "ECC_Pawn" "ECR_Overlap")
  (`self.SetIcon` (`self.Platform`)))

(fn `FinishAnimation`)

(fn `FinishReversing`)

(fn `Initialize`
  (bind _asbp_game_instance (cast `/Game/Game/BP_GameInstance` (`GameplayStatics.GetGameInstance`)))
  (set `self.GameInstanceReference` _asbp_game_instance)
  (set `self.InitialTransform` (`SceneComponent.K2_GetComponentToWorld` (`self.Platform`)))
  (`self.SetActivationBehaviour`)
  (`self.SetResetBehaviour`)
  (`self.SetVisible`))

(fn `PlayNewTrggerSound`
  (params (NewSound :type "SoundBase Object Reference") (StartTime :type "Float (double-precision)"))
  (bind _triggeraudio (`self.TriggerAudio`))
  (if (not (`/Game/Game/BP_GameInstance.Muted` (`self.GameInstanceReference`)))
    (`AudioComponent.SetSound` _triggeraudio NewSound)
    (`AudioComponent.Play` _triggeraudio StartTime)))

(fn `ReverseAnimation`
  (set `self.IsReversing` true)
  (`TimelineComponent.Reverse` (`self.Animation`)))

(fn `SetIcon`
  (params (Component :type "StaticMeshComponent Object Reference"))
  (if (`self.ShowIconAtStart`)
    (`PrimitiveComponent.SetMaterial` (`local.Component`) 1 (`self.IconMaterial`))
    (else
      (`PrimitiveComponent.SetMaterial` (`local.Component`) 1 (`self.BlankIconMaterial`)))))

(fn `SetOrientation`
  (params (Component :type "SceneComponent Object Reference"))
  (switch `/Game/Data/ENUMs/ENUM_Direction` (`self.Orientation`)
    (:`NewEnumerator1`
      (`self.SetXYRotation` Component 0.0 180.0))
    (:`NewEnumerator2`
      (`self.SetXYRotation` Component -90.0))
    (:`NewEnumerator3`
      (`self.SetXYRotation` Component 90.0))
    (:`NewEnumerator4`
      (`self.SetXYRotation` Component 0.0 -90.0))
    (:`NewEnumerator5`
      (`self.SetXYRotation` Component 0.0 90.0))))

(fn `SetVisible`
  (bind _platform (`self.Platform`))
  (if (`/Game/Game/BP_GameInstance.TrapsVisible` (`self.GameInstanceReference`))
    (`PrimitiveComponent.SetRenderCustomDepth` _platform true)
    (else
      (`PrimitiveComponent.SetRenderCustomDepth` _platform false))))

(fn `SetXYRotation`
  (params (Target :type "SceneComponent Object Reference") (X :type "Float (double-precision)") (Y :type "Float (double-precision)"))
  (`SceneComponent.K2_SetWorldRotation` Target (`KismetMathLibrary.MakeRotator` X Y) false false))

(fn `ToggleVisibility`
  (`|ExecutionSequence`
    (:`then_0`
      (if (not (`self.ShowPlatform`))
        (`/Game/Game/BP_Macros.DisableComponent` (`self.Platform`))))
    (:`then_1`
      (if (not (`self.ShowBillboard`))
        (`SceneComponent.SetVisibility` (`self.Icon`) false false)))))

(fn `UserConstructionScript`
  (`/Game/Game/BP_Macros.SetMeshAndMaterial` (`self.Platform`) (`self.PlatformMesh`) (`self.PlatformMaterial`)
    (:`__`
      (`self.SetIcon` (`self.Platform`))
      (`self.ToggleVisibility`)
      (`self.SetOrientation` (`self.Root`))
      (`SceneComponent.SetRelativeScale3D` (`self.StepTrigger`) (`self.StepTriggerSize`))
      (`SceneComponent.K2_AddRelativeLocation` (`self.StepTrigger`) (`self.StepTriggerOffset`) false false))))