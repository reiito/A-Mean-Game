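; BP_Checkpoint is a checkpoint flag that, when activated, can set the player's spawn point.
; Its construction script applies the configured flag mesh and material, and BeginPlay caches the first player's BP_PlayerController.
; Activate branches on Type: Real writes the root's world transform to the controller's PlayerSpawnPoint, while Weird calls an empty WeirdBehaviour stub.
; Debug "Hello" prints remain in Activate and SetCheckpoint.
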(event `self.Activate`
  (`KismetSystemLibrary.PrintString` "Hello")
  (switch `/Game/Data/ENUMs/ENUM_CheckpointType` (`self.Type`)
    (:`NewEnumerator1`
      (`self.SetCheckpoint`))
    (:`NewEnumerator2`
      (`self.WeirdBehaviour`))))

(event `self.ReceiveBeginPlay`
  (bind _asbp_player_controller (cast `/Game/Player/BP_PlayerController` (`GameplayStatics.GetPlayerController` 0)))
  (set `self.PlayerControllerReference` _asbp_player_controller))

(fn `SetCheckpoint`
  (set `/Game/Player/BP_PlayerController.PlayerSpawnPoint` (`SceneComponent.K2_GetComponentToWorld` (`self.Root`)) (`self.PlayerControllerReference`))
  (`KismetSystemLibrary.PrintString` "Hello"))

(fn `UserConstructionScript`
  (`parent.UserConstructionScript`)
  (`/Game/Game/BP_Macros.SetMeshAndMaterial` (`self.Flag`) (`self.FlagMesh`) (`self.FlagMaterial`)))

(fn `WeirdBehaviour`)