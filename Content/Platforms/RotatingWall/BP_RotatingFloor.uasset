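; Rotating wall-and-floor platform that activates when the player steps on its trigger while facing the wall.
; After a delay it disables player input and plays a raise timeline, which lifts the platform and then starts the inherited Animation timeline.
; That animation yaws the shared Axis to turn wall and floor together.
; On finish, the raise reverses and input returns; construction sets the wall's look and starting yaw.
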(event `self.StepTrigger.OnComponentBeginOverlap`
  (params (OverlappedComponent :type "PrimitiveComponent Object Reference") (OtherActor :type "Actor Object Reference") (OtherComp :type "PrimitiveComponent Object Reference") (OtherBodyIndex :type Integer) (bFromSweep :type Boolean) (SweepResult :type "HitResult Structure (by ref)"))
  ;[1 1 1] Rotating Wall activation
  ;;[1 1 1] Enable only when player faces wall
  (if (and (`/Game/Game/BP_Macros.IsPlayer` OtherActor) (not (`/Game/Game/BP_Macros.IsActiveTimeline` (`self.Animation`))) (`/Game/Game/BP_Macros.IsPlayerFacingComponent` (`self.Wall`)))
    ;;[1 1 1] Disable input and play animation
    (`KismetSystemLibrary.Delay` (`self.StepOnActivationDelay`))
    (`self.TogglePlayerInput` false)
    (`self.Activate`)))

(event `self.Animation__UpdateFunc`
  ;[1 1 1] Animations
  (`self.Rotate`))

(event `self.FinishAnimation`
  ;[1 1 1] Animations
  ;;[1 1 1] Enable input, re-enable overlaps
  (`parent.FinishAnimation`)
  (`TimelineComponent.Reverse` (`self.PlatformRaiseAnimation`))
  (`self.TogglePlayerInput` true))

(event `self.Activate`
  ;[1 1 1] Adding extra animation, platform raise
  (set `self.Activated` true)
  (set `self.IsReversing` false)
  (`TimelineComponent.Play` (`self.PlatformRaiseAnimation`)))

(event `self.ReceiveBeginPlay`
  ;[1 1 1] Setup additional animation
  (`parent.ReceiveBeginPlay`)
  (`/Game/Game/BP_Macros.SetupLerpTimeline` (`self.PlatformRaiseAnimation`) "/Game/Data/CURVEs/CURVE_LinearLerp.CURVE_LinearLerp" (`self.PlatformRaiseAnimationSpeed`)))

(fn `Rotate`
  (bind _startingrotation (`self.StartingRotation`))
  ;[1 1 1] Apply rotation to both wall and floor
  (`SceneComponent.K2_SetRelativeRotation` (`self.Axis`) (`KismetMathLibrary.MakeRotator` 0.0 0.0 (`KismetMathLibrary.Lerp` _startingrotation (+ _startingrotation (`self.Rotation`)) (`TimelineComponent.GetPlaybackPosition` (`self.Animation`)))) false false))

(fn `TogglePlayerInput`
  (params (InputEnabled :type Boolean))
  (bind _asbp_character (cast `/Game/Player/BP_Character` (`GameplayStatics.GetPlayerPawn` 0)))
  (`/Game/Player/BP_Character.ToggleInput` _asbp_character InputEnabled))

(fn `UserConstructionScript`
  (`parent.UserConstructionScript`)
  (`/Game/Game/BP_Macros.SetMeshAndMaterial` (`self.Wall`) (`self.WallMesh`) (`self.WallMaterial`)
    (:`__`
      (`SceneComponent.K2_SetRelativeRotation` (`self.Axis`) (`KismetMathLibrary.MakeRotator` 0.0 0.0 (`self.StartingRotation`)) false false))))