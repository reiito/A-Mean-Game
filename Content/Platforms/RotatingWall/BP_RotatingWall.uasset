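; Rotating wall platform that turns in yaw when player 0 steps on its trigger while facing it.
; On activation it disables input, auto-moves the character and picks the spin direction from the player's side, randomly if centered.
; An inherited Animation timeline drives rotation and material fade, while camera collision is set to overlap.
; When the animation finishes, input and triggers are restored, then after a delay camera blocking and opacity.
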(event `self.StepTrigger.OnComponentBeginOverlap`
  (params (OverlappedComponent :type "PrimitiveComponent Object Reference") (OtherActor :type "Actor Object Reference") (OtherComp :type "PrimitiveComponent Object Reference") (OtherBodyIndex :type Integer) (bFromSweep :type Boolean) (SweepResult :type "HitResult Structure (by ref)"))
  ;[1 1 1] Rotating Wall activation
  ;;[1 1 1] Enable only when player faces wall
  (if (and (`/Game/Game/BP_Macros.IsPlayer` OtherActor) (not (`/Game/Game/BP_Macros.IsActiveTimeline` (`self.Animation`))) (`/Game/Game/BP_Macros.IsPlayerFacingComponent` (`self.StepTrigger`)))
    (`/Engine/EditorBlueprintResources/StandardMacros.DoOnce` false :!label _label
      (:`Completed`
        (`self.ResetEndOverlap`)
        (`KismetSystemLibrary.Delay` (`self.StepOnActivationDelay`))
        ;;[1 1 1] Disable camera collision, make character automatically move forward and disable input (Rotation generated depending on character orientation)
        (`PrimitiveComponent.SetCollisionResponseToChannel` (`self.Platform`) "ECC_Camera" "ECR_Overlap")
        (bind _asbp_character (cast `/Game/Player/BP_Character` OtherActor))
        (`/Game/Player/BP_Character.AutoMoveCharacter` _asbp_character 0.5)
        (`self.DisableInput` (`GameplayStatics.GetPlayerPawn` 0) null)
        (`self.GenerateRotationOnPlayerOverlap`)
        (`self.Activate`)))))

(event `ResetBeginOverlap`
  ;[1 1 1] Rotating Wall activation
  ;;[1 1 1] Enable only when player faces wall
  (goto _label :!via `Reset`))

(event `self.StepTrigger.OnComponentEndOverlap`
  (params (OverlappedComponent :type "PrimitiveComponent Object Reference") (OtherActor :type "Actor Object Reference") (OtherComp :type "PrimitiveComponent Object Reference") (OtherBodyIndex :type Integer))
  ;[1 1 1] Rotating Wall activation
  ;;[1 1 1] Enable only when player faces wall
  (if (and (`/Game/Game/BP_Macros.IsPlayer` OtherActor) (`self.Retrigger`) (not (`/Game/Game/BP_Macros.IsActiveTimeline` (`self.Animation`))))
    (`/Engine/EditorBlueprintResources/StandardMacros.DoOnce` false :!label _label_2
      (:`Completed`
        (`self.ResetBeginOverlap`)))))

(event `ResetEndOverlap`
  ;[1 1 1] Rotating Wall activation
  ;;[1 1 1] Enable only when player faces wall
  (goto _label_2 :!via `Reset`))

(event `ResetOld`
  ;[1 1 1] Reverse wall animation and unlock overlaps
  (`TimelineComponent.Reverse` (`self.Animation`))
  (`self.ResetEndOverlap`)
  (`self.ResetBeginOverlap`))

(event `self.Animation__UpdateFunc`
  ;[1 1 1] Animations
  (`self.Rotate`)
  (`MaterialInstanceDynamic.SetScalarParameterValue` (`self.MaterialInstance`) "Fade" (`KismetMathLibrary.Lerp` (`self.DefaultOpacity`) 0.6 (`TimelineComponent.GetPlaybackPosition` (`self.Animation`)))))

(event `EnableRotatingWall`
  ;[1 1 1] Animations
  ;;[1 1 1] Enable input, disable push area and re-enable camera collision after brief period, also resetting opacity
  (`self.EnableInput` (`GameplayStatics.GetPlayerPawn` 0) null)
  (`self.ResetEndOverlap`)
  (`self.ResetBeginOverlap`)
  (`KismetSystemLibrary.Delay` 2.0)
  (`PrimitiveComponent.SetCollisionResponseToChannel` (`self.Platform`) "ECC_Camera" "ECR_Block")
  (`MaterialInstanceDynamic.SetScalarParameterValue` (`self.MaterialInstance`) "Fade" (`self.DefaultOpacity`)))

(event `self.FinishReversing`
  ;[1 1 1] Animations
  (`parent.FinishReversing`)
  (`self.EnableRotatingWall` :!label _label_3))

(event `self.FinishAnimation`
  ;[1 1 1] Animations
  (`parent.FinishAnimation`)
  (goto _label_3))

(fn `GenerateRotationOnPlayerOverlap`
  (locals (Result :type "Float (double-precision)"))
  (`/Game/Game/BP_Macros.PlayerPositionRelativeToComponent` (`self.StepTrigger`)
    (:`PlayerToRight`
      (set `self.Rotation` (* (`self.Rotation`) -1.0)))
    (:`PlayerAtCenter`
      (set `self.Rotation` (`/Game/Game/BP_Macros.SelectRandom` (`self.Rotation`) (* (`self.Rotation`) -1.0))))))

(fn `Rotate`
  (locals (End :type "Float (double-precision)"))
  (bind _startingrotation (`self.StartingRotation`))
  ;[1 1 1] Apply rotation
  (`SceneComponent.K2_SetRelativeRotation` (`self.Platform`) (`KismetMathLibrary.MakeRotator` 0.0 0.0 (`KismetMathLibrary.Lerp` _startingrotation (+ _startingrotation (`self.Rotation`)) (`TimelineComponent.GetPlaybackPosition` (`self.Animation`)))) false false))

(fn `UserConstructionScript`
  (`parent.UserConstructionScript`)
  (`SceneComponent.K2_SetRelativeRotation` (`self.Platform`) (`KismetMathLibrary.MakeRotator` 0.0 0.0 (`self.StartingRotation`)) false false)
  (`SceneComponent.K2_SetRelativeRotation` (`self.StepTrigger`) (`KismetMathLibrary.MakeRotator` 0.0 0.0 (`self.StartingRotation`)) false false)
  (bind _returnvalue (`PrimitiveComponent.CreateDynamicMaterialInstance` (`self.Platform`) 0 "/Game/Platforms/Fade/MAT_FadeEffect.MAT_FadeEffect"))
  (bind _output_get (set `self.MaterialInstance` _returnvalue))
  (`MaterialInstanceDynamic.SetTextureParameterValue` _output_get "Texture" (`self.WallTexture`)))