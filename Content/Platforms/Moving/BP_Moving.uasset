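; BP_Moving is a child platform Blueprint that slides a main platform and an optional connected secondary platform along configurable directions.
; Each platform's behaviour binds to a movement dispatcher, called on timeline updates to move it from its start position.
; When incapacitation is enabled, the secondary trigger ragdolls the player during animation and can make a blockage block physics bodies.
; Construction configures placement, direction arrows, trigger and blockage.
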(event `self.ReceiveBeginPlay`
  ;[1 1 1] Animation type to run
  (`parent.ReceiveBeginPlay`)
  (set `self.SecondaryPlatformStartPos` (`SceneComponent.K2_GetComponentLocation` (`self.SecondaryPlatform`)))
  (`self.AssignPlatformBehaviour`)
  (`self.AssignSecondaryPlatformBehaviour`))

(event `AssignPlatformBehaviour`
  ;[1 1 1] Stand platform and connected platform behaviours
  (if (`|EnumInequality` (`self.BaseBehaviour`) "NewEnumerator6")
    (add `self.PlatformMovement` (delegate `AddPlatformMovement`))))

(event `self.Animation__UpdateFunc`
  ;[1 1 1] Stand platform and connected platform behaviours
  ;;[1 1 1] Call behaviour on timeline
  (`self.PlatformMovement`))

(event `AddPlatformMovement`
  ;[1 1 1] Stand platform and connected platform behaviours
  (`self.MovePlatform` (`self.BaseBehaviour`)))

(event `AssignSecondaryPlatformBehaviour`
  ;[1 1 1] Stand platform and connected platform behaviours
  (if (`|EnumInequality` (`self.Behaviour`) "NewEnumerator6")
    (add `self.PlatformMovement` (delegate `AddSecondaryPlatformMovement`))))

(event `AddSecondaryPlatformMovement`
  ;[1 1 1] Stand platform and connected platform behaviours
  (`self.MovePlatform` (`self.Behaviour`) "NewEnumerator7"))

(event `self.SecondaryPlatformTrigger.OnComponentBeginOverlap`
  (params (OverlappedComponent :type "PrimitiveComponent Object Reference") (OtherActor :type "Actor Object Reference") (OtherComp :type "PrimitiveComponent Object Reference") (OtherBodyIndex :type Integer) (bFromSweep :type Boolean) (SweepResult :type "HitResult Structure (by ref)"))
  ;[1 1 1] Overlapping (Ragdoll if incapacitate on)
  (if (and (and (`/Game/Game/BP_Macros.IsPlayer` OtherActor) (`self.Incapacitate`)) (`/Game/Game/BP_Macros.IsActiveTimeline` (`self.Animation`)))
    (bind _asbp_character (cast `/Game/Player/BP_Character` OtherActor))
    (`/Game/Player/BP_Character.Ragdoll` _asbp_character)
    (`self.HitPlayer` self)
    (if (`self.UseBlockage`)
      (`PrimitiveComponent.SetCollisionResponseToChannel` (`self.Blockage`) "ECC_PhysicsBody" "ECR_Block"))))

(event `self.EnablePlatform`
  (`parent.EnablePlatform`)
  (`self.SetIcon` (`self.SecondaryPlatform`)))

(event `self.DisablePlatform`
  (`parent.DisablePlatform`)
  (`self.DeactivateIcon` (`self.SecondaryPlatform`)))

(event `self.SetVisible`
  (bind _secondaryplatform (`self.SecondaryPlatform`))
  (`parent.SetVisible`)
  (if (`/Game/Game/BP_GameInstance.TrapsVisible` (`self.GameInstanceReference`))
    (`PrimitiveComponent.SetRenderCustomDepth` _secondaryplatform true)
    (else
      (`PrimitiveComponent.SetRenderCustomDepth` _secondaryplatform false))))

(fn `MovePlatform`
  (params (Direction :type "/Game/Platforms/Moving/ENUM_MovementDirection Enum" :default "NewEnumerator6") (ComponentToMove :type "/Game/Platforms/Moving/ENUM_MovingComponent Enum" :default "NewEnumerator6"))
  (locals (InitialPosition :type "Vector Structure") (Component :type "StaticMeshComponent Object Reference") (DirectionVector :type "Vector Structure"))
  (bind _initialtransform_location (`KismetMathLibrary.BreakTransform` (`self.InitialTransform`)))
  (bind _initialposition (`local.InitialPosition`))
  ;[1 1 1] Determine direction vector
  (set `local.DirectionVector` (`/Game/Game/BP_Macros.DirectionToVector` Direction))
  ;[1 1 1] Apply movement to component
  (switch `/Game/Platforms/Moving/ENUM_MovingComponent` (`local.ComponentToMove`)
    (:`NewEnumerator6`
      (set `local.Component` (`self.Platform`))
      (set `local.InitialPosition` _initialtransform_location))
    (:`NewEnumerator7`
      (set `local.Component` (`self.SecondaryPlatform`))
      (set `local.InitialPosition` (`self.SecondaryPlatformStartPos`))))
  (`/Game/Game/BP_Macros.MoveComponent` (`local.Component`) _initialposition (+ _initialposition (* (`local.DirectionVector`) (`self.MoveDistance`))) (`self.Animation`)))

(fn `SetupPlatforms`
  (locals (StartPos :type "Vector Structure") (ArrowRotation :type "Float (double-precision)" :default 90.0))
  ;[1 1 1] Set facing arrow direction on platform
  (`SceneComponent.K2_SetRelativeRotation` (`self.PlatformMovingDirection`) (`KismetMathLibrary.Conv_VectorToRotator` (* (`/Game/Game/BP_Macros.DirectionToVector` (`self.BaseBehaviour`)) (`local.ArrowRotation`))) false false)
  ;[1 1 1] Apply parameters to secondary platform if visible
  (`/Game/Game/BP_Macros.SetMeshAndMaterial` (`self.SecondaryPlatform`) (`self.SecondaryPlatformModel`) (`self.SecondaryPlatformMaterial`)
    (:`__`
      (if (`self.HasSecondaryPlatform`)
        (set `local.StartPos` (* (`/Game/Game/BP_Macros.DirectionToVector` (`self.PositionOffset`)) (`self.DistanceApart`)))
        (`SceneComponent.K2_SetRelativeLocation` (`self.SecondaryPlatform`) (`local.StartPos`) false false)
        (`SceneComponent.K2_SetRelativeRotation` (`self.SecondaryPlatformMovingDirection`) (`KismetMathLibrary.Conv_VectorToRotator` (* (`/Game/Game/BP_Macros.DirectionToVector` (`self.Behaviour`)) (`local.ArrowRotation`))) false false)
        (else
          (`/Game/Game/BP_Macros.DisableComponent` (`self.SecondaryPlatform`)))))))

(fn `UserConstructionScript`
  (`parent.UserConstructionScript`)
  (`self.SetIcon` (`self.SecondaryPlatform`))
  (`self.SetupPlatforms`)
  (`SceneComponent.SetRelativeScale3D` (`self.SecondaryPlatformTrigger`) (`self.KillTriggerSize`))
  (`SceneComponent.K2_AddRelativeLocation` (`self.SecondaryPlatformTrigger`) (`self.KillTriggerSizeOffset`) false false)
  ;[1 1 1] Prevent character phasing through
  (if (`self.UseBlockage`)
    (`SceneComponent.SetVisibility` (`self.Blockage`) true false)
    (`SceneComponent.SetRelativeScale3D` (`self.Blockage`) (`self.BlockageSize`))
    (`SceneComponent.K2_SetRelativeLocation` (`self.Blockage`) (`self.BlockagePosition`) false false)))