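; Platform Blueprint for a killable platform, with an icon material that reflects whether it kills or incapacitates.
; It overrides SetIcon to show the incapacitate, normal or blank icon on material slot 1.
; Activation reveals icons that are hidden at start.
; CallHitPlayer gates both the hit sound on KillPlayerAudio and its onward hit call behind the game instance's mute flag.
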(event `self.ReceiveBeginPlay`
  (`parent.ReceiveBeginPlay`))

(event `self.Activate`
  (`parent.Activate`)
  (`self.ActivateIcon` (`self.Platform`)))

(event `self.SetIcon`
  (params (Component :type "StaticMeshComponent Object Reference"))
  ;[1 1 1] Override set icon to take into consideration whether incapacitate is on or off
  (if (`self.ShowIconAtStart`)
    (if (`self.Incapacitate`)
      (`PrimitiveComponent.SetMaterial` Component 1 (`self.IncapacitateMaterial`))
      (else
        (`PrimitiveComponent.SetMaterial` Component 1 (`self.IconMaterial`))))
    (else
      (`PrimitiveComponent.SetMaterial` Component 1 (`self.BlankIconMaterial`)))))

(fn `ActivateIcon`
  (params (Component :type "StaticMeshComponent Object Reference"))
  (if (not (`self.ShowIconAtStart`))
    (if (`self.Incapacitate`)
      (`PrimitiveComponent.SetMaterial` (`local.Component`) 1 (`self.IncapacitateMaterial`))
      (else
        (`PrimitiveComponent.SetMaterial` (`local.Component`) 1 (`self.IconMaterial`))))))

(fn `CallHitPlayer`
  (if (not (`/Game/Game/BP_GameInstance.Muted` (`self.GameInstanceReference`)))
    (`self.PlayNewHitSound` (`self.HitSound`))
    (`self.HitPlayer` self)))

(fn `PlayNewHitSound`
  (params (NewSound :type "SoundBase Object Reference") (StartTime :type "Float (double-precision)"))
  (bind _killplayeraudio (`self.KillPlayerAudio`))
  (`AudioComponent.SetSound` _killplayeraudio NewSound)
  (`AudioComponent.Play` _killplayeraudio StartTime))

(fn `UserConstructionScript`
  (`parent.UserConstructionScript`))