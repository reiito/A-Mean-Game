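; Spike trap, built on a parent Blueprint, that ragdolls and impales the player on contact when incapacitation is enabled.
; The parent's animation drives the spikes' Z position, with spike and trigger collision enabled on activation and disabled after reversing.
; Hits lock the character after a delay, releasing it for certain activation behaviors; spikes left triggered also push the hips downward.
; A game-instance setting toggles custom-depth rendering for trap visibility.
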(event `self.Animation__UpdateFunc`
  ;[1 1 1] Spike animation
  (`SceneComponent.K2_SetRelativeLocation` (`self.Spikes`) (`KismetMathLibrary.MakeVector` 0.0 0.0 (`KismetMathLibrary.Lerp` (`self.InitialPosition`) (`self.EndPosition`) (`TimelineComponent.GetPlaybackPosition` (`self.Animation`)))) false false))

(event `self.Activate`
  ;[1 1 1] Activation and deactivation
  (`parent.Activate`)
  (`self.EnableSpikes`))

(event `self.FinishReversing`
  ;[1 1 1] Activation and deactivation
  (`parent.FinishReversing`)
  (`self.DisableSpikes`))

(event `self.SpikeTrigger.OnComponentBeginOverlap`
  (params (OverlappedComponent :type "PrimitiveComponent Object Reference") (OtherActor :type "Actor Object Reference") (OtherComp :type "PrimitiveComponent Object Reference") (OtherBodyIndex :type Integer) (bFromSweep :type Boolean) (SweepResult :type "HitResult Structure (by ref)"))
  (bind _activationbehavior (`self.ActivationBehavior`))
  ;[1 1 1] Overlapping spikes
  (if (and (`/Game/Game/BP_Macros.IsPlayer` OtherActor) (`self.Incapacitate`))
    (bind _asbp_character (cast `/Game/Player/BP_Character` OtherActor))
    (`/Game/Player/BP_Character.Ragdoll` _asbp_character)
    (`self.CallHitPlayer`)
    (if (`self.TriggeredNotReset`)
      (set `self.ImpaleDelay` 0.3)
      (`PrimitiveComponent.AddForce` (`Character.Mesh` _asbp_character) (0.0 0.0 -200000.0) "Hips" true))
    (`KismetSystemLibrary.Delay` (`self.ImpaleDelay`))
    (`/Game/Player/BP_Character.LockPosition` _asbp_character)
    (if (or (`|EnumEquality` _activationbehavior "NewEnumerator2") (`|EnumEquality` _activationbehavior "NewEnumerator3") (`|EnumEquality` _activationbehavior "NewEnumerator1"))
      (`KismetSystemLibrary.Delay` (/ (`TimelineComponent.GetPlayRate` (`self.Animation`)) 48.0))
      (`/Game/Player/BP_Character.UnlockPosition` _asbp_character)
      (elif (`|EnumEquality` (`self.ResetBehaviour`) "NewEnumerator2")
        (`/Engine/EditorBlueprintResources/StandardMacros.DoOnce` false
          (:`Completed`
            (set `self.TriggeredNotReset` true)))))))

(event `self.SetVisible`
  (bind _spikes (`self.Spikes`))
  (`parent.SetVisible`)
  (if (`/Game/Game/BP_GameInstance.TrapsVisible` (`self.GameInstanceReference`))
    (`PrimitiveComponent.SetRenderCustomDepth` _spikes true)
    (else
      (`PrimitiveComponent.SetRenderCustomDepth` _spikes false))))

(fn `DisableSpikes`
  (`/Game/Game/BP_Macros.DisableComponent` (`self.Spikes`)
    (:`__`
      (`/Game/Game/BP_Macros.DisableComponent` (`self.SpikeTrigger`)))))

(fn `EnableSpikes`
  (`/Game/Game/BP_Macros.EnableComponent` (`self.Spikes`) "QueryAndPhysics"
    (:`__`
      (`/Game/Game/BP_Macros.EnableComponent` (`self.SpikeTrigger`) "QueryOnly"))))

(fn `SetSpikeTrigger`
  (bind (_returnvalue_origin _returnvalue_boxextent) (`KismetMathLibrary.BreakBoxSphereBounds` (`StaticMesh.GetBounds` (`StaticMeshComponent.StaticMesh` (`self.Spikes`)))))
  (`|ExecutionSequence`
    (:`then_0`
      (if (`self.TriggerSizeToMeshSize`)
        (`BoxComponent.SetBoxExtent` (`self.SpikeTrigger`) _returnvalue_boxextent false)))
    (:`then_1`
      (`SceneComponent.K2_AddRelativeLocation` (`self.SpikeTrigger`) (`self.SpikeTriggerPositionOffset`) false false))))

(fn `UserConstructionScript`
  (`parent.UserConstructionScript`)
  (`/Game/Game/BP_Macros.SetMeshAndMaterial` (`self.Spikes`) (`self.SpikesMesh`) (`self.SpikesMaterial`)
    (:`__`
      (`SceneComponent.K2_SetRelativeLocation` (`self.Spikes`) (`KismetMathLibrary.MakeVector` 0.0 0.0 (`self.InitialPosition`)) false false)
      (`self.SetSpikeTrigger`)
      (`self.DisableSpikes`))))