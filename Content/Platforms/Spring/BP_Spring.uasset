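; Spring platform, built on a parent platform class, that launches the player along the spring's up direction and can optionally incapacitate them.
; A timeline animates the spring's height, and overlapping its trigger during that animation launches the character, gated by a DoOnce.
; With Incapacitate set, it also ragdolls the character, adds a scaled force and reports the hit.
; Parent overrides enable the spring on activation, then disable it and reset the gate after reversing.
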(event `self.Animation__UpdateFunc`
  ;[1 1 1] Spring animation
  (`/Game/Game/BP_Macros.MoveComponent` (`self.Spring`) (`KismetMathLibrary.MakeVector` 0.0 0.0 (`self.InitialPosition`)) (`KismetMathLibrary.MakeVector` 0.0 0.0 (+ (`self.InitialPosition`) (`self.Distance`))) (`self.Animation`) true))

(event `self.SpringTrigger.OnComponentBeginOverlap`
  (params (OverlappedComponent :type "PrimitiveComponent Object Reference") (OtherActor :type "Actor Object Reference") (OtherComp :type "PrimitiveComponent Object Reference") (OtherBodyIndex :type Integer) (bFromSweep :type Boolean) (SweepResult :type "HitResult Structure (by ref)"))
  ;[1 1 1] Player hitting spring, send them upwards, kill if incapacitate is on
  (if (and (`/Game/Game/BP_Macros.IsPlayer` OtherActor) (`/Game/Game/BP_Macros.IsActiveTimeline` (`self.Animation`)))
    (`/Engine/EditorBlueprintResources/StandardMacros.DoOnce` false :!label _label
      (:`Completed`
        (bind _asbp_character (cast `/Game/Player/BP_Character` OtherActor))
        (bind _returnvalue (+ (`self.GetActorForwardVector` _asbp_character) (* (`SceneComponent.GetUpVector` (`self.Spring`)) (* (`self.Strength`) 1000.0))))
        (`Character.LaunchCharacter` _asbp_character _returnvalue false false)
        (if (`self.Incapacitate`)
          (`/Game/Player/BP_Character.Ragdoll` _asbp_character)
          (`PrimitiveComponent.AddForce` (`Character.Mesh` _asbp_character) (* _returnvalue (* 1000.0 (`self.DeathLaunchStrength`))) "None" false)
          (`self.CallHitPlayer`))))))

(event `self.FinishReversing`
  ;[1 1 1] Parent overridden events
  (`parent.FinishReversing`)
  (`/Game/Game/BP_Macros.DisableComponent` (`self.Spring`)
    (:`__`
      (goto _label :!via `Reset`))))

(event `self.Activate`
  ;[1 1 1] Parent overridden events
  (`parent.Activate`)
  (`/Game/Game/BP_Macros.EnableComponent` (`self.Spring`) "QueryAndPhysics"))

(event `self.DisablePlatform`
  (`parent.DisablePlatform`)
  (`self.DeactivateIcon` (`self.Spring`)))

(fn `UserConstructionScript`
  (bind _spring (`self.Spring`))
  (`parent.UserConstructionScript`)
  (`self.SetIcon` (`self.Spring`))
  (`/Game/Game/BP_Macros.SetMeshAndMaterial` _spring (`self.SpringMesh`) (`self.SpringMaterial`)
    (:`__`
      (`/Game/Game/BP_Macros.DisableComponent` _spring
        (:`__`
          (`SceneComponent.K2_SetRelativeLocation` _spring (`KismetMathLibrary.MakeVector` 0.0 0.0 (`self.InitialPosition`)) false false))))))