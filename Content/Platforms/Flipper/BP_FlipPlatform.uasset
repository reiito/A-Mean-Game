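; Platform variant with a flipper that swings out on activation and can ragdoll the player it hits.
; Construction sets the flipper's model, material, icon and facing, and enables the kill trigger only when Incapacitate is set.
; The inherited animation drives the roll, and the flipper hides again after reversing or completing a full-turn rotation.
; Hits count only while the animation is active, and can turn on an optional Blockage against physics bodies.
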(event `self.AnimationUpdate`
  ;[1 1 1] Flipper behaviour
  (`SceneComponent.K2_SetRelativeRotation` (`self.Flipper`) (`KismetMathLibrary.MakeRotator` (`KismetMathLibrary.Lerp` 0.0 (`self.Rotation`) (`TimelineComponent.GetPlaybackPosition` (`self.Animation`)))) false false))

(event `self.Activate`
  ;[1 1 1] Flipper behaviour
  (`parent.Activate`)
  (`SceneComponent.SetVisibility` (`self.FlipperMesh`) true false))

(event `self.DisablePlatform`
  ;[1 1 1] Enabling/Disabling behaviour extension
  (`parent.DisablePlatform`)
  (`self.DeactivateIcon` (`self.FlipperMesh`)))

(event `self.FinishAnimation`
  ;[1 1 1] Enabling/Disabling behaviour extension
  (`self.IsFullRotation`
    (:`FullRotation`
      (`SceneComponent.SetVisibility` (`self.FlipperMesh`) false false :!label _label))))

(event `self.FinishReversing`
  ;[1 1 1] Enabling/Disabling behaviour extension
  (goto _label))

(event `self.EnablePlatform`
  ;[1 1 1] Enabling/Disabling behaviour extension
  (`parent.EnablePlatform`)
  (`self.SetIcon` (`self.FlipperMesh`)))

(event `self.KillTrigger.OnComponentBeginOverlap`
  (params (OverlappedComponent :type "PrimitiveComponent Object Reference") (OtherActor :type "Actor Object Reference") (OtherComp :type "PrimitiveComponent Object Reference") (OtherBodyIndex :type Integer) (bFromSweep :type Boolean) (SweepResult :type "HitResult Structure (by ref)"))
  ;[1 1 1] Killing player
  (if (`/Game/Game/BP_Macros.IsActiveTimeline` (`self.Animation`))
    (bind _asbp_character (cast `/Game/Player/BP_Character` OtherActor))
    (`/Game/Player/BP_Character.Ragdoll` _asbp_character)
    (`self.CallHitPlayer`)
    (if (`self.UseBlockage`)
      (`PrimitiveComponent.SetCollisionResponseToChannel` (`self.Blockage`) "ECC_PhysicsBody" "ECR_Block"))))

(fn `SetupFlipper`
  (`|ExecutionSequence`
    (:`then_0`
      ;[1 1 1] Setup flipper materials and model
      (`StaticMeshComponent.SetStaticMesh` (`self.FlipperMesh`) (`self.FlipperModel`))
      (`PrimitiveComponent.SetMaterial` (`self.FlipperMesh`) 0 (`self.FlipperMaterial`))
      (`self.SetIcon` (`self.FlipperMesh`))
      (`SceneComponent.SetVisibility` (`self.FlipperMesh`) false false))
    (:`then_1`
      ;[1 1 1] Check if incapacitate, toggle overlapping behaviour of trigger
      (if (`self.Incapacitate`)
        (`PrimitiveComponent.SetCollisionResponseToChannel` (`self.KillTrigger`) "ECC_Pawn" "ECR_Overlap")
        (else
          (`PrimitiveComponent.SetCollisionResponseToChannel` (`self.KillTrigger`) "ECC_Pawn" "ECR_Ignore"))))
    (:`then_2`
      ;[1 1 1] Orient flipper
      (switch `/Game/Platforms/Flipper/ENUM_FlipperPosition` (`self.FlipperPosition`)
        (:`NewEnumerator0`
          (`SceneComponent.K2_SetRelativeRotation` (`self.FlipperStartOrientation`) (struct :`Yaw` 90.0) false false))
        (:`NewEnumerator1`
          (`SceneComponent.K2_SetRelativeRotation` (`self.FlipperStartOrientation`) (struct :`Yaw` -90.0) false false))
        (:`NewEnumerator3`
          (`SceneComponent.K2_SetRelativeRotation` (`self.FlipperStartOrientation`) (struct :`Yaw` 180.0) false false))))))

(fn `UserConstructionScript`
  (`parent.UserConstructionScript`)
  (`self.SetupFlipper`)
  ;[1 1 1] Show blockage in editor
  (if (`self.UseBlockage`)
    (`SceneComponent.SetVisibility` (`self.Blockage`) true false)))