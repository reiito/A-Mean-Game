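; BP_TrapDoor is a trap door platform, built on a parent platform Blueprint, with two panels that swing in opposite directions.
; The animation update rolls the Axis and AxisL pivots up to 90 degrees in mirrored directions, using the Animation playback position as the lerp alpha.
; Enable, disable and construction extend the parent logic to PlatformL, handling its icon and, at construction, its mesh and material.
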(event `self.Animation__UpdateFunc`
  (bind _returnvalue (`TimelineComponent.GetPlaybackPosition` (`self.Animation`)))
  (`SceneComponent.K2_SetRelativeRotation` (`self.Axis`) (`KismetMathLibrary.MakeRotator` (`KismetMathLibrary.Lerp` 0.0 -90.0 _returnvalue)) false false)
  (`SceneComponent.K2_SetRelativeRotation` (`self.AxisL`) (`KismetMathLibrary.MakeRotator` (`KismetMathLibrary.Lerp` 0.0 90.0 _returnvalue)) false false))

(event `self.DisablePlatform`
  (`parent.DisablePlatform`)
  (`self.DeactivateIcon` (`self.PlatformL`)))

(event `self.EnablePlatform`
  (`parent.EnablePlatform`)
  (`self.SetIcon` (`self.PlatformL`)))

(fn `UserConstructionScript`
  (`parent.UserConstructionScript`)
  (`self.SetIcon` (`self.PlatformL`))
  (`/Game/Game/BP_Macros.SetMeshAndMaterial` (`self.PlatformL`) (`self.PlatformMesh`) (`self.PlatformMaterial`)))