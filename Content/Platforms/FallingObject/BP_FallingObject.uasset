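; Falling-object hazard platform that drops a physics block when the player steps on its trigger or on play, crushing the character it hits if set to incapacitate.
; The death trigger turns on for each drop and off when the block hits anything but the player.
; CatchArea handles retrigger, loop or trigger-once behaviour, optionally spawning a capped number of left-behind copies.
; Overrides parent reset events to return the block or stop its physics.
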(event `self.StepTrigger.OnComponentBeginOverlap`
  (params (OverlappedComponent :type "PrimitiveComponent Object Reference") (OtherActor :type "Actor Object Reference") (OtherComp :type "PrimitiveComponent Object Reference") (OtherBodyIndex :type Integer) (bFromSweep :type Boolean) (SweepResult :type "HitResult Structure (by ref)"))
  ;[1 1 1] Check player overlap
  (if (`/Game/Game/BP_Macros.IsPlayer` OtherActor)
    (`KismetSystemLibrary.Delay` (`self.StepOnActivationDelay`))
    (`self.DropObject`)))

(event `self.DeathTrigger.OnComponentBeginOverlap`
  (params (OverlappedComponent :type "PrimitiveComponent Object Reference") (OtherActor :type "Actor Object Reference") (OtherComp :type "PrimitiveComponent Object Reference") (OtherBodyIndex :type Integer) (bFromSweep :type Boolean) (SweepResult :type "HitResult Structure (by ref)"))
  ;[1 1 1] Kill when overlapping
  (bind _asbp_character (cast `/Game/Player/BP_Character` OtherActor))
  (if (`self.Incapacitate`)
    (`/Game/Player/BP_Character.Crush` _asbp_character)))

(event `self.ReceiveBeginPlay`
  ;[1 1 1] Store block's initial position
  (`self.AddRotationOffset`)
  (set `self.ObjectStartLocation` (`SceneComponent.K2_GetComponentToWorld` (`self.FallingObject`)))
  (`parent.ReceiveBeginPlay`)
  (if (`self.ActivateOnPlay`)
    (`self.DropObject`)))

(event `DropObject`
  ;[1 1 1] Activation
  (`|ExecutionSequence`
    (:`then_0`
      (if (not (`self.VisibleBeforeTrigger`))
        (`self.SetObjectVisibility` true)))
    (:`then_1`
      (if (not (`self.InheritSpeedOnRetrigger`))
        (`PrimitiveComponent.SetAllPhysicsLinearVelocity` (`self.FallingObject`) (0.0 0.0 0.0) false)))
    (:`then_2`
      (set `self.Activated` true)
      (`SceneComponent.K2_SetWorldTransform` (`self.FallingObject`) (`self.ObjectStartLocation`) false true)
      (`self.EnableDeathTrigger`)
      (`PrimitiveComponent.SetSimulatePhysics` (`self.FallingObject`) true))))

(event `self.JumpToInitialStateOnReset`
  ;[1 1 1] Overidden behaviour
  ;;[1 1 1] Re-enabling - Do same behaviour for both re-enable events
  (add `self.Reset` (delegate `ReturnObjectToStartOnReset`)))

(event `self.StopOnReset`
  ;[1 1 1] Overidden behaviour
  ;;[1 1 1] Instead of stopping timeline, stop simulating physics
  (add `self.Reset` (delegate `StopFallingObject`)))

(event `ReturnObjectToStartOnReset`
  ;[1 1 1] Overidden behaviour
  ;;[1 1 1] Re-enabling - Do same behaviour for both re-enable events
  (`self.ReturnObjectToStart`))

(event `StopFallingObject`
  ;[1 1 1] Overidden behaviour
  ;;[1 1 1] Instead of stopping timeline, stop simulating physics
  (`PrimitiveComponent.SetSimulatePhysics` (`self.FallingObject`) false)
  (`PrimitiveComponent.SetCollisionResponseToAllChannels` (`self.DeathTrigger`) "ECR_Ignore")
  (`PrimitiveComponent.SetCollisionResponseToChannel` (`self.StepTrigger`) "ECC_Pawn" "ECR_Ignore")
  (`self.DeactivateIcon` (`self.Platform`)))

(event `self.ReverseAnimationOnReset`
  ;[1 1 1] Overidden behaviour
  ;;[1 1 1] Re-enabling - Do same behaviour for both re-enable events
  (add `self.Reset` (delegate `ReturnObjectToStartOnReset`)))

(event `self.FallingObject.OnComponentHit`
  (params (HitComponent :type "PrimitiveComponent Object Reference") (OtherActor :type "Actor Object Reference") (OtherComp :type "PrimitiveComponent Object Reference") (NormalImpulse :type "Vector Structure") (Hit :type "HitResult Structure (by ref)"))
  ;[1 1 1] Object hitting anything besides player, disable its death trigger
  (if (not (`/Game/Game/BP_Macros.IsPlayer` OtherActor))
    (`self.DisableDeathTrigger`)))

(event `self.CatchArea.OnComponentBeginOverlap`
  (params (OverlappedComponent :type "PrimitiveComponent Object Reference") (OtherActor :type "Actor Object Reference") (OtherComp :type "PrimitiveComponent Object Reference") (OtherBodyIndex :type Integer) (bFromSweep :type Boolean) (SweepResult :type "HitResult Structure (by ref)"))
  ;[1 1 1] Object passed floor trigger. Extra behaviour dependant on activation behaviour
  (if (`self.IsFallingObject` OtherComp)
    (switch `/Game/Platforms/ENUM_ActivationBehaviour` (`self.ActivationBehavior`)
      (:`NewEnumerator2`
        (`KismetSystemLibrary.Delay` (`self.AnimationFinishDelay`))
        (`self.UpdateObjectLastPosition`)
        (`self.LeaveObjectBehind`))
      (:`NewEnumerator3`
        (`KismetSystemLibrary.Delay` (`self.LoopIterationDelay`))
        (`self.UpdateObjectLastPosition`)
        (`self.LeaveObjectBehind`)
        (`self.DropObject`))
      (:`NewEnumerator0`
        (`self.DisablePlatform` :!label _label))
      (:`NewEnumerator1`
        (goto _label)))))

(fn `AddRotationOffset`
  (locals (AddedRotation :type "Float (double-precision)"))
  (if (`self.AddRandomRotationOffset`)
    (`SceneComponent.K2_AddLocalRotation` (`self.FallingObject`) (`KismetMathLibrary.MakeRotator` (`KismetMathLibrary.RandomFloatInRange` (* (`self.RotationOffset`) -1.0) (`self.RotationOffset`))) false false)))

(fn `DisableDeathTrigger`
  (`PrimitiveComponent.SetCollisionResponseToChannel` (`self.DeathTrigger`) "ECC_PhysicsBody" "ECR_Ignore")
  (`PrimitiveComponent.SetCollisionResponseToChannel` (`self.DeathTrigger`) "ECC_Pawn" "ECR_Ignore"))

(fn `EnableDeathTrigger`
  (`PrimitiveComponent.SetCollisionResponseToChannel` (`self.DeathTrigger`) "ECC_PhysicsBody" "ECR_Overlap")
  (`PrimitiveComponent.SetCollisionResponseToChannel` (`self.DeathTrigger`) "ECC_Pawn" "ECR_Overlap"))

(fn `LeaveObjectBehind`
  (if (and (`self.LeaveObjectsBehind`) (< (`self.ObjectCount`) (`self.MaxObjectCount`)))
    (`SceneComponent.K2_SetWorldTransform` (`self.FallingObject`) (`self.ObjectStartLocation`) false true)
    (`PrimitiveComponent.SetSimulatePhysics` (`self.FallingObject`) false)
    (`|SpawnActorFromClass` "/Game/Platforms/FallingObject/BP_LeftBehindObject.BP_LeftBehindObject_C" (`self.ObjectLastPosition`) "Undefined" "OverrideRootScale" null null)
    (`/Engine/EditorBlueprintResources/StandardMacros.IncrementInt` (`self.ObjectCount`))))

(fn `ReturnObjectToStart`
  (if (`|EnumInequality` (`self.ActivationBehavior`) "NewEnumerator3")
    (`PrimitiveComponent.SetSimulatePhysics` (`self.FallingObject`) false)
    (`self.SetObjectVisibility` (`self.VisibleBeforeTrigger`))
    (`self.UpdateObjectLastPosition`)
    (`self.LeaveObjectBehind`)
    (`SceneComponent.K2_SetWorldTransform` (`self.FallingObject`) (`self.ObjectStartLocation`) false false)))

(fn `SetObjectVisibility`
  (params (Visible :type Boolean))
  (if Visible
    (`/Game/Game/BP_Macros.EnableComponent` (`self.FallingObject`) "QueryAndPhysics")
    (else
      (`/Game/Game/BP_Macros.DisableComponent` (`self.FallingObject`)))))

(fn `UpdateObjectLastPosition`
  (if (`self.LeaveObjectsBehind`)
    (set `self.ObjectLastPosition` (`SceneComponent.K2_GetComponentToWorld` (`self.FallingObject`)))))

(fn `UserConstructionScript`
  (`parent.UserConstructionScript`)
  (`/Game/Game/BP_Macros.SetMeshAndMaterial` (`self.FallingObject`) (`self.BlockMesh`) (`self.BlockMaterial`)
    (:`__`
      (`SceneComponent.K2_AddRelativeLocation` (`self.FallingObject`) (`KismetMathLibrary.MakeVector` 0.0 0.0 (`self.ObjectPosition`)) false false)
      (`SceneComponent.SetRelativeScale3D` (`self.CatchArea`) (`self.CatchAreaSize`))
      (`SceneComponent.SetRelativeScale3D` (`self.FallingObject`) (`self.FallingObjectSize`))
      (if (not (`self.VisibleBeforeTrigger`))
        (`self.SetObjectVisibility` false)))))